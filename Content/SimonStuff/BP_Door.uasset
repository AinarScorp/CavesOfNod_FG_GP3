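; BP_Door is a door that opens when its linked Sigil completes.
; BeginPlay stores the start location, creates a dynamic material with emissive off, and binds Open to the Sigil's completion event.
; Open runs a timeline that sweeps the actor toward an offset from its start position.
; Each timeline update also turns the emissive on and plays the door sound at the actor's location.
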(event `open`
  (bind _startposition (`self.StartPosition`))
  (bind (_direction _newtrack_0) (`Timeline|Opening Timeline` :!via `PlayFromStart`)
    (:`Update`
      (`self.K2_SetActorLocation` (`KismetMathLibrary.VLerp` _startposition (+ _startposition (`self.OpenPosition`)) _newtrack_0) true)
      (`MaterialInstanceDynamic.SetScalarParameterValue` (`self.Material`) (`self.EmissiveParameter`) 1.0)
      (`GameplayStatics.PlaySoundAtLocation` "/Game/_Game/Sounds/MetaSounds/SFX_DoorSound.SFX_DoorSound" (`self.K2_GetActorLocation`) (struct) 1.0 1.0 0.0 null null null null))))

(event `self.ReceiveBeginPlay`
  (bind _returnvalue (`PrimitiveComponent.CreateDynamicMaterialInstance` (`self.StaticMesh`) 0 null (`self.EmissiveParameter`)))
  (bind _output_get (set `self.Material` _returnvalue))
  (`MaterialInstanceDynamic.SetScalarParameterValue` _output_get (`self.EmissiveParameter`) 0.0)
  (set `self.StartPosition` (`self.K2_GetActorLocation`))
  (add `/Game/SimonStuff/art/paintminigame/BP_PaintBoard.Sigil Complete` (`self.Sigil`) (delegate `open`)))

(fn `UserConstructionScript`)