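; BP_BigRockBossKillah is a rock actor carrying five Eggsplosive child actors, apparently for killing a boss, judging by its name.
; Its Activate event waits briefly, then stops physics simulation on the static mesh.
; It then makes each child actor component visible and sets that Eggsplosive's respawn point to its current location, so respawns follow where the rock ended up.
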(event `Activate`
  (`KismetSystemLibrary.Delay` 5.0)
  (`PrimitiveComponent.SetSimulatePhysics` (`self.StaticMeshComponent`) false)
  (for _array_element (`|MakeArray` (`self.BP_Eggsplosive1`) (`self.BP_Eggsplosive`) (`self.BP_Eggsplosive5`) (`self.BP_Eggsplosive2`) (`self.BP_Eggsplosive3`))
    (`SceneComponent.SetVisibility` _array_element true false)
    (bind _asbp_eggsplosive (cast `/Game/_Game/Blueprints/Actors/BP_Eggsplosive` (`ChildActorComponent.ChildActor` _array_element)))
    (bind _returnvalue (`self.K2_GetActorLocation` _asbp_eggsplosive))
    (`self.K2_SetActorLocation` _asbp_eggsplosive _returnvalue false false)
    (set `/Game/_Game/Blueprints/Actors/BP_Eggsplosive.RespawnPoint` _returnvalue _asbp_eggsplosive)))

(fn `UserConstructionScript`)