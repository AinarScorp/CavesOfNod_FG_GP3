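; Paint minigame board that players paint with hits to complete a sigil.
; GetHit traces the impact to find its UV, draws a stencil material into a render target there and spawns a splatter effect.
; Six hittable boxes, bound on BeginPlay and also carrying one-shot projectile overlaps, track progress.
; At six counted hits it signals sigil completion, lights the material, clears the paint, blocks further drawing and plays a sound.
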(event `Clear Board`
  (`KismetRenderingLibrary.ClearRenderTarget2D` (`self.Texture Render Target`) :!label _label))

(event `self.ReceiveBeginPlay`
  (`self.BindEveryColliderToOnHitEvent`)
  (bind _returnvalue (`KismetMaterialLibrary.CreateDynamicMaterialInstance` (`self.meterial`)))
  (bind _output_get (set `self.MainMAT` _returnvalue))
  (`PrimitiveComponent.SetMaterial` (`self.Canvas`) 0 _output_get)
  (bind _returnvalue_2 (`KismetMaterialLibrary.CreateDynamicMaterialInstance` "/Game/SimonStuff/art/paintminigame/MAT_PaintStencil.MAT_PaintStencil"))
  (set `self.Stencil` _returnvalue_2)
  (goto _label))

(event `DrawOnBoard`
  (params (`Location to Draw` :type "Vector2D Structure"))
  (bind _stencil (`self.Stencil`))
  (if (not (`self.completed`))
    (`MaterialInstanceDynamic.SetVectorParameterValue` _stencil "DrawLocation" (`KismetMathLibrary.Conv_VectorToLinearColor` (`KismetMathLibrary.Conv_Vector2DToVector` `Location to Draw` 0.1)))
    (`KismetRenderingLibrary.DrawMaterialToRenderTarget` (`self.Texture Render Target`) _stencil)))

(event `DrawSize`)

(event `self.GetHit`
  (params (DamageAmount :type "Float (single-precision)") (EventInstigator :type "Controller Object Reference") (DamageCauser :type "Actor Object Reference") (Hit :type "HitResult Structure (by ref)"))
  (bind (_bblockinghit _binitialoverlap _time _distance _location _impactpoint _normal _impactnormal) (`GameplayStatics.BreakHitResult` Hit))
  (bind _outhit (`KismetSystemLibrary.LineTraceSingle` :`Start` (+ _impactpoint (* _impactnormal 10.0)) :`End` (+ _impactpoint (* _impactnormal -10.0)) :`TraceChannel` "TraceTypeQuery1" :`bIgnoreSelf` false))
  (`self.DrawOnBoard` (`GameplayStatics.FindCollisionUV` _outhit))
  (`NiagaraFunctionLibrary.SpawnSystemAtLocation` "/Game/_Game/VFX/FX_Splatter.FX_Splatter" (`EinarLibrary.GetRaycastHitLocation` _outhit) (struct) (0.1 0.1 0.1)))

(event `self.BP_BoxHittable.OnComponentBeginOverlap`
  (params (OverlappedComponent :type "PrimitiveComponent Object Reference") (OtherActor :type "Actor Object Reference") (OtherComp :type "PrimitiveComponent Object Reference") (OtherBodyIndex :type Integer) (bFromSweep :type Boolean) (SweepResult :type "HitResult Structure (by ref)"))
  ;[1 1 1] To Delete if using raycast
  (cast `/Game/_Game/Blueprints/Actors/BP_FirstPersonProjectile` OtherActor)
  (`/Engine/EditorBlueprintResources/StandardMacros.DoOnce` false
    (:`Completed`
      (`self.OnHitCollider` :!label _label_2))))

(event `self.BP_BoxHittable1.OnComponentBeginOverlap`
  (params (OverlappedComponent :type "PrimitiveComponent Object Reference") (OtherActor :type "Actor Object Reference") (OtherComp :type "PrimitiveComponent Object Reference") (OtherBodyIndex :type Integer) (bFromSweep :type Boolean) (SweepResult :type "HitResult Structure (by ref)"))
  ;[1 1 1] To Delete if using raycast
  (cast `/Game/_Game/Blueprints/Actors/BP_FirstPersonProjectile` OtherActor)
  (`/Engine/EditorBlueprintResources/StandardMacros.DoOnce` false
    (:`Completed`
      (goto _label_2))))

(event `self.BP_BoxHittable2.OnComponentBeginOverlap`
  (params (OverlappedComponent :type "PrimitiveComponent Object Reference") (OtherActor :type "Actor Object Reference") (OtherComp :type "PrimitiveComponent Object Reference") (OtherBodyIndex :type Integer) (bFromSweep :type Boolean) (SweepResult :type "HitResult Structure (by ref)"))
  ;[1 1 1] To Delete if using raycast
  (cast `/Game/_Game/Blueprints/Actors/BP_FirstPersonProjectile` OtherActor)
  (`/Engine/EditorBlueprintResources/StandardMacros.DoOnce` false
    (:`Completed`
      (goto _label_2))))

(event `self.BP_BoxHittable3.OnComponentBeginOverlap`
  (params (OverlappedComponent :type "PrimitiveComponent Object Reference") (OtherActor :type "Actor Object Reference") (OtherComp :type "PrimitiveComponent Object Reference") (OtherBodyIndex :type Integer) (bFromSweep :type Boolean) (SweepResult :type "HitResult Structure (by ref)"))
  ;[1 1 1] To Delete if using raycast
  (cast `/Game/_Game/Blueprints/Actors/BP_FirstPersonProjectile` OtherActor)
  (`/Engine/EditorBlueprintResources/StandardMacros.DoOnce` false
    (:`Completed`
      (goto _label_2))))

(event `self.BP_BoxHittable4.OnComponentBeginOverlap`
  (params (OverlappedComponent :type "PrimitiveComponent Object Reference") (OtherActor :type "Actor Object Reference") (OtherComp :type "PrimitiveComponent Object Reference") (OtherBodyIndex :type Integer) (bFromSweep :type Boolean) (SweepResult :type "HitResult Structure (by ref)"))
  ;[1 1 1] To Delete if using raycast
  (cast `/Game/_Game/Blueprints/Actors/BP_FirstPersonProjectile` OtherActor)
  (`/Engine/EditorBlueprintResources/StandardMacros.DoOnce` false
    (:`Completed`
      (goto _label_2))))

(event `self.BP_BoxHittable5.OnComponentBeginOverlap`
  (params (OverlappedComponent :type "PrimitiveComponent Object Reference") (OtherActor :type "Actor Object Reference") (OtherComp :type "PrimitiveComponent Object Reference") (OtherBodyIndex :type Integer) (bFromSweep :type Boolean) (SweepResult :type "HitResult Structure (by ref)"))
  ;[1 1 1] To Delete if using raycast
  (cast `/Game/_Game/Blueprints/Actors/BP_FirstPersonProjectile` OtherActor)
  (`/Engine/EditorBlueprintResources/StandardMacros.DoOnce` false
    (:`Completed`
      (goto _label_2))))

(fn `BindEveryColliderToOnHitEvent`
  (for _array_element (`|MakeArray` (`self.BP_BoxHittable2`) (`self.BP_BoxHittable3`) (`self.BP_BoxHittable4`) (`self.BP_BoxHittable5`) (`self.BP_BoxHittable`) (`self.BP_BoxHittable1`))
    (add `/Game/_Game/Blueprints/Components/Collisions/BP_BoxHittable.TheBoxGotHIt` _array_element (`|CreateDelegate` :!event `OnHitCollider`))))

(fn `BP_PaintBoard_AutoGenFunc`
  (params (HitResult :type "HitResult Structure")))

(fn `OnHitCollider`
  (bind _result (`/Engine/EditorBlueprintResources/StandardMacros.IncrementInt` (`self.hits`))
    (:`  `
      (`/Engine/EditorBlueprintResources/StandardMacros.CompareInt` _result 6
        (:`>`
          _)
        (:`==`
          _))
      (`self.Sigil Complete`)
      (`MaterialInstanceDynamic.SetScalarParameterValue` (`self.MainMAT`) "Completed" 1.0)
      (`self.Clear Board`)
      (set `self.completed` true)
      (`GameplayStatics.PlaySoundAtLocation` "/Game/_Game/Sounds/MetaSounds/SFX_SigilLit.SFX_SigilLit" (`self.K2_GetActorLocation`) (struct) 1.0 1.0 0.0 null null null null))))

(fn `UserConstructionScript`)