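; BP_BigDoor is a door that opens once two linked sigils, left and right, are both completed.
; Each sigil's completion event lights its emissive dynamic material; the left also plays a voice line, the right streams in the CorridorEnemies level instance.
; With both unlocked, a timeline lerps the actor by an offset, replaying the door sound and enabling pawn overlap on the final-door voice-line collider every update.
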(event `open lock 1`
  (set `self.UnlockLeft` true)
  (`self.OpenDoor`)
  (`MaterialInstanceDynamic.SetScalarParameterValue` (`self.MaterialSigilOne`) (`self.EmissiveParameter`) 1.0)
  (`GameplayStatics.PlaySound2D` (`self.VoiceLine`) 1.0 1.0 0.0 null null))

(event `self.ReceiveBeginPlay`
  (bind _returnvalue (`PrimitiveComponent.CreateDynamicMaterialInstance` (`self.StaticMesh`) 0 null (`self.EmissiveParameter`)))
  (bind _output_get (set `self.MaterialSigilOne` _returnvalue))
  (`MaterialInstanceDynamic.SetScalarParameterValue` _output_get (`self.EmissiveParameter`) 0.0)
  (bind _returnvalue_2 (`PrimitiveComponent.CreateDynamicMaterialInstance` (`self.StaticMesh1`) 0 null (`self.EmissiveParameter`)))
  (bind _output_get_2 (set `self.MaterialSigilTwo` _returnvalue_2))
  (`MaterialInstanceDynamic.SetScalarParameterValue` _output_get_2 (`self.EmissiveParameter`) 0.0)
  (set `self.StartPosition` (`self.K2_GetActorLocation`))
  (add `/Game/SimonStuff/art/paintminigame/BP_PaintBoard.Sigil Complete` (`self.SigilLeft`) (delegate `open lock 1`))
  (add `/Game/SimonStuff/art/paintminigame/BP_PaintBoard.Sigil Complete` (`self.SigilRight`) (delegate `Open lock 2`)))

(event `Open lock 2`
  (set `self.UnlockRight` true)
  (`LevelStreamingDynamic.LoadLevelInstanceBySoftObjectPtr` "/Game/_Game/Levels/Main/CorridorEnemies.CorridorEnemies" (0.0 0.0 0.0) (struct) "" null)
  (`self.OpenDoor`)
  (`MaterialInstanceDynamic.SetScalarParameterValue` (`self.MaterialSigilTwo`) (`self.EmissiveParameter`) 1.0))

(event `OpenDoor`
  (bind _startposition (`self.StartPosition`))
  (if (and (`self.UnlockRight`) (`self.UnlockLeft`))
    (bind (_direction _newtrack_0) (`Timeline|Opening Timeline` :!via `PlayFromStart`)
      (:`Update`
        (`self.K2_SetActorLocation` (`KismetMathLibrary.VLerp` _startposition (+ _startposition (`self.OpenPosition`)) _newtrack_0) true)
        (`GameplayStatics.PlaySoundAtLocation` "/Game/_Game/Sounds/MetaSounds/SFX_DoorSound.SFX_DoorSound" (`self.K2_GetActorLocation`) (struct) 1.0 1.0 0.0 null null null null)
        (bind _returnvalue (`GameplayStatics.GetActorOfClass` "/Game/_Game/Blueprints/Actors/VoiceLinesTriggers/BP_FinalDoorVoiceLineCollider.BP_FinalDoorVoiceLineCollider_C"))
        (`PrimitiveComponent.SetCollisionResponseToChannel` (`/Game/_Game/Blueprints/Actors/VoiceLinesTriggers/BP_FinalDoorVoiceLineCollider.Box` _returnvalue) "ECC_Pawn" "ECR_Overlap")))))

(fn `UserConstructionScript`)