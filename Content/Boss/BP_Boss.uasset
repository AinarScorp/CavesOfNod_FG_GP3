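; Boss enemy that, whenever idle, randomly picks on Tick between a leg stab and a spit attack.
; Stab picks the leg on the player's side or the surviving one, blends montages with Control Rig targeting, damages overlapped actors and raises the leg via timeline.
; Spit launches a player-aimed projectile from the mouth on a montage notify, and replaces stab when no legs remain.
; Weakspot leg-damage and death logic is present but disconnected.
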(event OnComponentHit(Sphere1)
  (params (HitComponent :type Primitive%20Component%20Object%20Reference) (OtherActor :type Actor%20Object%20Reference) (OtherComp :type Primitive%20Component%20Object%20Reference) (NormalImpulse :type Vector :default "0, 0, 0") (Hit :type Hit%20Result%20Structure%20%28by%20ref%29)))

(event OnComponentHit(Sphere)
  (params (HitComponent :type Primitive%20Component%20Object%20Reference) (OtherActor :type Actor%20Object%20Reference) (OtherComp :type Primitive%20Component%20Object%20Reference) (NormalImpulse :type Vector :default "0, 0, 0") (Hit :type Hit%20Result%20Structure%20%28by%20ref%29)))

(event Custom|Stab%20Attack
  ;[1 1 1] Stab Attack
  ;;[1 1 1] still have legs left
  (Math|Integer|CompareInt (+ (Variables|Default|GetLeft%20Leg%20Health) (Variables|Default|GetRight%20Leg%20Health))
    (:>
      ;;[1 1 1] reset legs
      (bind _output_get (Variables|Default|SetRight%20Leg%20Position "0, 0, 0"))
      (Variables|Default|SetLeft%20Leg%20Position _output_get)
      ;;[1 1 1] Windup
      (Variables|Default|SetAttackSide (.Is%20On%20Right%20Side (CallFunction|GetPlayerLocation)))
      (Animation|Montage|PlayMontage (Variables|Default|GetBoss) "/Game/Boss/Animations/Boss_AttackMontage.Boss_AttackMontage" 1.0 0.0 (select (Variables|Default|GetAttackSide) "StabRight" "StabLeft")
        (:then
          (Variables|Default|SetUse%20CtrlRig true))
        (:OnCompleted
          (bind _outactors (Collision|SphereOverlapActors (Variables|Default|GetAttack%20Position) 0.0 (Utilities|Array|MakeArray "ObjectTypeQuery3") 0))
          (for _array_element _outactors
            (Game|Damage|ApplyDamage (.AsTP%20First%20Person%20Character (Utilities|Casting|CastToTP_FirstPersonCharacter _array_element)) 5e+01 0 0)))
        (:OnBlendOut
          ;;[1 1 1] set leg position to player
          (bind _output_get_2 (Variables|Default|SetAttack%20Position (.Location (CallFunction|GetPlayerLocation))))
          (if (Variables|Default|GetAttackSide)
            (Variables|Default|SetRight%20Leg%20Position _output_get_2)
            (else
              (Variables|Default|SetLeft%20Leg%20Position _output_get_2)))
          (Utilities|FlowControl|Delay 3.0)
          ;;[1 1 1] return leg
          (bind _alpha (Timeline|Leg%20Raise PlayFromStart)
            (:Update
              (if (Variables|Default|GetAttackSide)
                (Variables|Default|SetRight%20Leg%20Position (Math|Vector|Lerp(Vector) (Variables|Default|GetAttack%20Position) (Math|Vector|MakeVector (.x (Variables|Default|GetAttack%20Position)) (.y (Variables|Default|GetAttack%20Position)) (+ (.z (Variables|Default|GetAttack%20Position)) 1e+02)) _alpha))
                (else
                  (Variables|Default|SetLeft%20Leg%20Position (Math|Vector|Lerp(Vector) (Variables|Default|GetAttack%20Position) (Math|Vector|MakeVector (.x (Variables|Default|GetAttack%20Position)) (.y (Variables|Default|GetAttack%20Position)) (+ (.z (Variables|Default|GetAttack%20Position)) 1e+02)) _alpha)))))
            (:Finished
              (Animation|Montage|PlayMontage (Variables|Default|GetBoss) "/Game/Boss/Animations/Boss_AttackMontage.Boss_AttackMontage" 1.0 0.0 "LToDefault"
                (:then
                  (Variables|Default|SetUse%20CtrlRig false))
                (:OnCompleted
                  (Variables|Default|SetisPerforming false))))))))
    (:==
      (CallFunction|SpitAttack :!label _label))
    (:<
      (goto _label))))

(event Custom|Spit%20Attack
  (bind _boss (Variables|Default|GetBoss))
  (bind _returnvalue (Transformation|GetSocketLocation _boss "Mouth"))
  ;[1 1 1] Spit Attack
  (Animation|Montage|PlayMontage (Variables|Default|GetBoss) "/Game/Boss/Animations/Boss_AttackMontage.Boss_AttackMontage" 1.0 0.0 "Spit"
    (:OnCompleted
      (Variables|Default|SetisPerforming false))
    (:OnNotifyBegin
      (Game|SpawnActorfromClass "/Game/Boss/Attack_Assets/BP_BossProjectile.BP_BossProjectile_C" (Math|Transform|MakeTransform _returnvalue (Math|Rotator|MakeRotfromX (Math|Vector|GetUnitDirection(Vector) _returnvalue (Transformation|GetActorLocation (Game|Player|GetPlayerPawn 0)))) "1.000000,1.000000,1.000000") "Undefined" 0 0))))

(event Custom|Bump%20Attack)

(event EventBeginPlay
  ;[1 1 1] Setup
)

(event EventTick
  (params (DeltaSeconds :type Float%20%28single-precision%29))
  ;[1 1 1] Attack select
  (if (not (Variables|Default|GetisPerforming))
    (Variables|Default|SetisPerforming true)
    (switch int (Math|Random|RandomIntegerinRange 0 1)
      (:0
        (CallFunction|StabAttack))
      (:1
        (CallFunction|SpitAttack)))))

(event Input|KeyboardEvents|DebugKeyTab
  (params (Key :type Key%20Structure :default "None") (ActionValue :type Input%20Action%20Value%20Structure))
  ;[1 1 1] Stab Attack
  (:Pressed
    (CallFunction|StabAttack)))

(event Input|KeyboardEvents|DebugKeyQ
  (params (Key :type Key%20Structure :default "None") (ActionValue :type Input%20Action%20Value%20Structure))
  ;[1 1 1] Spit Attack
  (:Pressed
    (CallFunction|SpitAttack)))

(fn ConstructionScript)

(fn GetPlayerLocation
  (bind _returnvalue (Game|Player|GetPlayerPawn 0))
  (bind _returnvalue_2 (Transformation|GetActorLocation _returnvalue))
  ;[1 1 1] if both legs are alive
  (if (and (> (Variables|Default|GetRight%20Leg%20Health) 0) (> (Variables|Default|GetLeft%20Leg%20Health) 0))
    ;[1 1 1] Find location and choose leg
    (Math|Float|CompareFloat (Class|KismetMathLibrary|DegAcos (Math|Vector|DotProduct (Transformation|GetActorRightVector) (Math|Vector|Normalize (- _returnvalue_2 (Transformation|GetActorLocation))))) 9e+01
      (:>
        (return false _returnvalue_2))
      (:==
        _)
      (:<
        _))
    (return true _returnvalue_2)
    (else
      ;[1 1 1] return the legs thats alive
      (return (> (Variables|Default|GetRight%20Leg%20Health) 0) _returnvalue_2))))