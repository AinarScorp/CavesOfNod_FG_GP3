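; BP_HittableSphere is a hittable collision sphere that acts as a target requiring a set number of hits.
; Each GetHit event increments a hit counter and spawns a small weak-point explosion effect at the impact point while below the threshold.
; Reaching the threshold fires the SphereGotHIt dispatcher with itself and spawns a different explosion effect, gated by a DoOnce so it happens only once.
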(event `self.GetHit`
  (params (DamageAmount :type "Float (single-precision)") (EventInstigator :type "Controller Object Reference") (DamageCauser :type "Actor Object Reference") (Hit :type "HitResult Structure (by ref)"))
  (bind (_bblockinghit _binitialoverlap _time _distance _location _impactpoint) (`GameplayStatics.BreakHitResult` Hit))
  (bind _result (`/Engine/EditorBlueprintResources/StandardMacros.IncrementInt` (`self.NumberOfHitsTaken`))
    (:`  `
      (if (>= _result (`self.NumberOfHitsRequired`))
        (`/Engine/EditorBlueprintResources/StandardMacros.DoOnce` false
          (:`Completed`
            (`self.SphereGotHIt` self)
            (`NiagaraFunctionLibrary.SpawnSystemAtLocation` "/Game/_Game/VFX/FX_Explotion.FX_Explotion" _impactpoint (struct) (0.1 0.1 0.1))))
        (else
          (`NiagaraFunctionLibrary.SpawnSystemAtLocation` "/Game/_Game/VFX/FX_ExplotionWeakPoint.FX_ExplotionWeakPoint" _impactpoint (struct) (0.1 0.1 0.1)))))))