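; BP_Recoil adds random first-person camera recoil when the shoot input fires.
; Each IA_ShootFP Triggered event applies a random negative pitch input and a small random yaw input to either side.
; It first runs an invisible Visibility multi-line trace from the camera, whose end offset keeps only the scaled Z of the forward vector and whose hits are unused.
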(event `EnhancedInput|/Game/_Game/Inputs/Actions/IA_ShootFP`
  (params (ActionValue :type Boolean) (ElapsedSeconds :type "Float (double-precision)") (TriggeredSeconds :type "Float (double-precision)") (InputAction :type "InputAction Object Reference" :default "/Game/_Game/Inputs/Actions/IA_ShootFP.IA_ShootFP"))
  (bind _firstpersoncameracomponent (`self.FirstPersonCameraComponent`))
  (bind _returnvalue (`SceneComponent.K2_GetComponentLocation` _firstpersoncameracomponent))
  (:`Triggered`
    (`KismetSystemLibrary.LineTraceMulti` _returnvalue (+ _returnvalue (* (`KismetMathLibrary.GetForwardVector` (`SceneComponent.K2_GetComponentRotation` _firstpersoncameracomponent)) (0.0 0.0 100.0))) "TraceTypeQuery1")
    (`Pawn.AddControllerPitchInput` (`KismetMathLibrary.RandomFloatInRange` -1.0 -2.0))
    (`Pawn.AddControllerYawInput` (`KismetMathLibrary.RandomFloatInRange` 0.1 -0.1))))

(event `self.ReceiveBeginPlay`)