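; BP_Rifle is the rifle weapon component, handling firing, stabbing and egg throwing.
; Fire throws an egg, falling back to the parent fire logic when none is held; starting a stab with an egg throws it instead.
; Shooting and stabbing play sections of one first-person montage on Mesh1P, and ending fire stops the character's rifle recoil.
; Wall hits spawn a small splatter Niagara effect at the impact point.
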(event `self.ReceiveTick`
  (params (DeltaSeconds :type "Float (single-precision)")))

(event `self.OnFire`
  ;[1 0.7339 0.02011] Fire/shoot
  (`|PlayMontage` (`self.Mesh1P`) "/Game/myWeapon/Rifle_Actions_montage.Rifle_Actions_montage" 1.0 0.0 "Default"))

(event `self.HitWall`
  (params (HitResult :type "HitResult Structure"))
  (`NiagaraFunctionLibrary.SpawnSystemAtLocation` "/Game/_Game/VFX/FX_Splatter.FX_Splatter" (`EinarLibrary.GetRaycastHitLocation` HitResult) (struct) (0.1 0.1 0.1)))

(event `self.OnEndFire`
  ;[1 0.7339 0.02011] Fire/shoot
  (`/Game/_Game/Blueprints/Characters/BP_FirstPersonCharacter.End Rifle Recoil` (`self.CharacterRef`)))

(event `self.Fire`
  ;[1 0.7339 0.02011] Fire/shoot
  (`self.ThrowEgg`
    (:`NoEgg`
      (`parent.Fire`))))

(event `self.OnBeginStab`
  (if (`self.hasEgg`)
    (`self.ThrowEgg`)
    (else
      (`|PlayMontage` (`self.Mesh1P`) "/Game/myWeapon/Rifle_Actions_montage.Rifle_Actions_montage" 2.0 0.0 "stab"))))

(event `self.OnEndStab`
  (`|PlayMontage` (`self.Mesh1P`) "/Game/myWeapon/Rifle_Actions_montage.Rifle_Actions_montage" 1.0 0.0 "stabend"))

(event `self.StabButtonReleased`
  (`parent.StabButtonReleased`)
  (`self.OnEndStab`))