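; Path tracer component that probes the surface around its cached enemy with raycast triplets.
; ShootRaycasts first fires two forward traces and one right trace, storing them as closer, further and right hits.
; If any miss, it retries with angled traces rotated from the movement-down vector around the enemy's right axis, plus a sideways-offset third.
; It returns true only when a full triplet hits, with optional color-coded debug drawing.
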(fn `ShootRaycasts`
  (returns (SuccessfulHit :type Boolean))
  (locals (RotatedVector :type "Vector Structure" :default (0.0 0.0 0.0)))
  (bind (_outhitresult _successfulhit) (`self.RaycastForward` 1000.0 (struct :`R` 0.913099 :`G` 1.0 :`B` 0.039546 :`A` 1.0) (`self.RayCastLength`) (`self.DrawRaycasts`)))
  (if _successfulhit
    (bind (_outhitresult_2 _successfulhit_2) (`self.RaycastForward` 1100.0 (struct :`R` 0.064803 :`G` 0.078187 :`B` 1.0 :`A` 1.0) (`self.RayCastLength`) (`self.DrawRaycasts`)))
    (if _successfulhit_2
      (bind (_outhitresult_3 _successfulhit_3) (`self.RaycastRight` 1000.0 (struct :`R` 1.0 :`G` 0.027321 :`B` 0.768151 :`A` 1.0) (`self.RayCastLength`) (`self.DrawRaycasts`)))
      (if _successfulhit_3
        (set `self.HitRight` _outhitresult_3)
        (set `self.HitForwardCloser` _outhitresult)
        (set `self.HitForwardFurther` _outhitresult_2)
        (return true)
        (else
          (bind (_outhitresult_4 _successfulhit_4 _rotatedvector) (`self.RaycastFromForwardTillAngledDown` 120.0 (`self.GetMovementDirectionDown` 1000.0) (`Actor.GetActorRightVector` (`self.CachedEnemy`)) (struct :`R` 0.027321 :`G` 0.496933 :`B` 0.73791 :`A` 1.0) (`self.RayCastLengthAroundAngle`) (`self.DrawRaycasts`) :!label _label))
          (if _successfulhit_4
            (set `local.RotatedVector` _rotatedvector)
            (bind (_outhitresult_5 _successfulhit_5) (`self.RaycastFromForwardTillAngledDown` 118.0 (`self.GetMovementDirectionDown` 1000.0) (`Actor.GetActorRightVector` (`self.CachedEnemy`)) (struct :`R` 1.0 :`G` 0.090842 :`B` 0.896269 :`A` 1.0) (`self.RayCastLengthAroundAngle`) (`self.DrawRaycasts`)))
            (if _successfulhit_5
              (bind (_outhitresult_6 _successfulhit_6) (`self.RaycastFromForwardTillAngledDown` 5.0 (`local.RotatedVector`) (`self.GetMovementDirectionDown` 1000.0) (struct :`R` 0.023153 :`G` 0.051269 :`B` 0.617207 :`A` 1.0) (`self.RayCastLengthAroundAngleRight`) (`self.DrawRaycasts`)))
              (if _successfulhit_6
                (set `self.HitRight` _outhitresult_6)
                (set `self.HitForwardCloser` _outhitresult_4)
                (set `self.HitForwardFurther` _outhitresult_5)
                (return true)
                (else
                  _))))))
      (else
        (goto _label)))
    (else
      (goto _label)))
  (return false))