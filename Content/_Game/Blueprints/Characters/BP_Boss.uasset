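; Boss actor that repeatedly stabs at the player, choosing a leg by player side or remaining limb.
; Stab montages set leg positions and a Control Rig flag, with an indicator and sphere-trace hit check.
; Sigil events reveal weak points, whose destruction spawns aggravated support enemies and eventually detaches that limb via physics.
; Losing both limbs triggers death: a boulder sequence plays and a destructible egg attaches to the mouth.
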(event `self.ReceiveBeginPlay`
  ;[0.7843 0.04416 1] BeginPlay
  (`self.AttachCollidersToSockets`)
  (`self.Subscribe to Leg Weak Points`)
  (`self.AssignHPForWeakPoints`)
  (`self.ToggleWeakPoints` false true true)
  (`self.BindEventsToSigilsComplete`)
  (`KismetSystemLibrary.Delay` 5.0)
  (`self.SpawnAttackIndicator`)
  (`self.Stab Attack`))

(event `Make Lost Limb Disappear`
  (params (BoneName :type Name))
  ;[1 0.7909 0.07902] LimbDisappearAfterSomeTime TODO: Turn off the collision of the detached limb
  (`KismetSystemLibrary.Delay` 5.0)
  (`SkinnedMeshComponent.HideBoneByName` (`self.Boss`) BoneName "PBO_None"))

(event `Die`
  (`KismetSystemLibrary.Delay` 1.0)
  (`self.PlayBoulderSequence`)
  (set `self.Is Dead` true)
  (`|PlayMontage` (`self.Boss`) "/Game/SimonStuff/Stuff/Animations/Boss_StabAttack.Boss_StabAttack"
    (:`then`
      (`self.SetDestuctibleInMouth`))))

(event `Stab Attack`
  (bind (_is_on_right_side _location) (`self.Get Player LocationForAttack`))
  (bind _attack_position (`self.Attack Position`))
  (bind (_returnvalue_x _returnvalue_y) (`KismetMathLibrary.BreakVector` (`KismetMathLibrary.SelectVector` (`self.Right Leg Position`) (`self.Left Leg Position`) (`self.AttackSide`))))
  ;[0.2329 1 0] Attack Logic
  (if (`self.CanAttack`)
    (set `self.AttackSide` _is_on_right_side)
    (set `self.Attack Position` (`KismetMathLibrary.MakeVector` (.x _location) (.y _location) (+ (.z _location) -120.0)))
    (`|PlayMontage` (`self.Boss`) "/Game/SimonStuff/Stuff/Animations/Boss_StabAttack.Boss_StabAttack" 1.0 0.0 (select `bool` (`self.AttackSide`) :`false` "Lattack" :`true` "Rattack" :!type "Name")
      (:`then`
        (`self.HandleIndicator` false)
        (if (`self.AttackSide`)
          (set `self.Right Leg Position` _attack_position)
          (else
            (set `self.Left Leg Position` _attack_position))))
      (:`OnCompleted`
        (`NiagaraFunctionLibrary.SpawnSystemAtLocation` "/Game/SimonStuff/Stuff/explotion/P_Destruction_Concrete_Converted_2.P_Destruction_Concrete_Converted_2" (`KismetMathLibrary.MakeVector` _returnvalue_x _returnvalue_y))
        (`self.HandleIndicator` true))
      (:`OnBlendOut`
        (set `self.use ctrl rig` true)
        (`KismetSystemLibrary.Delay` 1.0)
        (`self.Reset stab`)))))

(event `Reset stab`
  ;[0.2329 1 0] Attack Logic
  (`|PlayMontage` (`self.Boss`) "/Game/SimonStuff/Stuff/Animations/Boss_StabAttack.Boss_StabAttack" 1.0 0.0 (select `bool` (`self.AttackSide`) :`false` "lRecover" :`true` "rRecover" :!type "Name")
    (:`OnCompleted`
      (`KismetSystemLibrary.Delay` 0.5)
      (`self.Stab Attack`))
    (:`OnBlendOut`
      (set `self.Right Leg Position` (0.0 0.0 0.0))
      (set `self.Left Leg Position` (0.0 0.0 0.0))
      (set `self.use ctrl rig` false))))

(event `PerformAttack`
  (bind _actualattacklocation (`self.ActualAttackLocation`))
  ;[1 0.01458 0] PlayerDamage
  (bind _outhits (`KismetSystemLibrary.SphereTraceMultiForObjects` _actualattacklocation _actualattacklocation 150.0 (`self.ObjectTypesForAttack`)))
  (for _array_element _outhits
    (message `/Game/_Game/Interfaces/BPI_BossHittable.GetHitByBoss` (`.HitActor` (`GameplayStatics.BreakHitResult` _array_element)) self)))

(fn `AssignHPForWeakPoints`
  (for _array_element (`self.AllWeakPoints`)
    (set `/Game/_Game/Blueprints/Components/Collisions/BP_HittableSphere.NumberOfHitsRequired` (`self.NumberOfHitsRequiredForTheWeakPoint`) _array_element)))

(fn `AttachCollidersToSockets`
  (`|ExecutionSequence`
    (:`then_0`
      (`SceneComponent.K2_AttachToComponent` (`self.RightLegUp`) (`self.Boss`) (`self.GetArmName` false true) "KeepWorld" "KeepWorld" "KeepWorld" true))
    (:`then_1`
      (`SceneComponent.K2_AttachToComponent` (`self.RightLegDown`) (`self.Boss`) (`self.GetArmName` false) "KeepWorld" "KeepWorld" "KeepWorld" true))
    (:`then_2`
      (`SceneComponent.K2_AttachToComponent` (`self.LeftLegDown`) (`self.Boss`) (`self.GetArmName` true) "KeepWorld" "KeepWorld" "KeepWorld" true))
    (:`then_3`
      (`SceneComponent.K2_AttachToComponent` (`self.LeftLegUp`) (`self.Boss`) (`self.GetArmName` true true) "KeepWorld" "KeepWorld" "KeepWorld" true))))

(fn `BindEventsToSigilsComplete`
  (bind _rightsigil (`self.RightSigil`)
    (:`then`
      (add `/Game/SimonStuff/art/paintminigame/BP_PaintBoard.Sigil Complete` _rightsigil (`|CreateDelegate` :!event `ShowLeftLegWeakPoints`)))
    (:`else`
      _))
  (bind _leftsigil (`self.LeftSigil`)
    (:`then`
      (add `/Game/SimonStuff/art/paintminigame/BP_PaintBoard.Sigil Complete` _leftsigil (`|CreateDelegate` :!event `ShowRightLegWeakPoints`)))
    (:`else`)))

(fn `CanAttack`
  (returns (NewParam :type Boolean))
  (return (not (or (`self.Is Dead`) (and (`self.LostRightLimb`) (`self.LostLeftLimb`))))))

(fn `DestroyLeftWeakPoint`
  (params (DestroyedSphere :type "/Game/_Game/Blueprints/Components/Collisions/BP_HittableSphere Object Reference"))
  (`self.DestroyThisComponentAndChildren` DestroyedSphere)
  (bind _result (`/Engine/EditorBlueprintResources/StandardMacros.IncrementInt` (`self.LeftWeakPointDamaged`))
    (:`  `
      (`/Engine/EditorBlueprintResources/StandardMacros.CompareInt` _result (`self.AmountOfLeftWeakPoints`)
        (:`>`
          _)
        (:`==`
          _))
      (`self.LoseLimb` true))))

(fn `DestroyRightWeakPoint`
  (params (DestroyedSphere :type "/Game/_Game/Blueprints/Components/Collisions/BP_HittableSphere Object Reference"))
  (`self.DestroyThisComponentAndChildren` DestroyedSphere)
  (bind _result (`/Engine/EditorBlueprintResources/StandardMacros.IncrementInt` (`self.RightWeakPointDamaged`))
    (:`  `
      (`/Engine/EditorBlueprintResources/StandardMacros.CompareInt` _result (`self.AmountOfRightWeakPoints`)
        (:`>`
          _)
        (:`==`
          _))
      (`self.LoseLimb` false))))

(fn `DestroyThisComponentAndChildren`
  (params (SphereComp :type "/Game/_Game/Blueprints/Components/Collisions/BP_HittableSphere Object Reference"))
  (`self.SummonSupport` (`/Game/_Game/Blueprints/Components/Collisions/BP_HittableSphere.IsOnLeftSide` SphereComp) true (`SceneComponent.K2_GetComponentLocation` SphereComp))
  (for _array_element (`SceneComponent.GetChildrenComponents` SphereComp true)
    (`ActorComponent.K2_DestroyComponent` _array_element))
  (`ActorComponent.K2_DestroyComponent` SphereComp))

(fn `DissolveThisActor`
  (bind _boss (`self.Boss`))
  (`PrimitiveComponent.SetCollisionEnabled` (`self.Boss`) "NoCollision")
  (`NiagaraFunctionLibrary.SpawnSystemAttached` "/Game/_Game/VFX/FX_Dissolve.FX_Dissolve" _boss "None" (`SceneComponent.K2_GetComponentLocation` _boss) (struct) "KeepRelativeOffset")
  (`SceneComponent.SetHiddenInGame` _boss true false)
  (`LightComponent.SetIntensity` (`PointLight.PointLightComponent` (`self.LightPath`)) 10.0)
  (`ActorComponent.K2_DestroyComponent` (`self.Box`)))

(fn `Get Player LocationForAttack`
  (returns (`Is On Right Side` :type Boolean) (Location :type "Vector Structure"))
  (bind _returnvalue (`self.K2_GetActorLocation` (`GameplayStatics.GetPlayerPawn` 0)))
  (if (or (`self.LostRightLimb`) (`self.LostLeftLimb`))
    (return (`self.LostLeftLimb`) _returnvalue)
    (else
      (return (<= (`EinarLibrary.GetAngleDegBetweenVectors` (`self.GetActorRightVector`) (`KismetMathLibrary.Normal` (- (`self.K2_GetActorLocation` (`GameplayStatics.GetPlayerPawn` 0)) (`self.K2_GetActorLocation`)))) 90.0) _returnvalue))))

(fn `GetArmName`
  (params (GetLeftArm :type Boolean) (GetUpArm :type Boolean))
  (returns (ArmName :type Name))
  (if GetLeftArm
    (return (select `bool` GetUpArm :`false` "Toe_L" :`true` "ArmDown_L" :!type "Name"))
    (else
      (return (select `bool` GetUpArm :`false` "Toe_R" :`true` "ArmDown_R" :!type "Name")))))

(fn `HandleIndicator`
  (params (SetHidden :type Boolean) (LocationOffsetFromPlayer :type "Vector Structure" :default (0.0 0.0 90.0)))
  (bind _attackindicator (`self.AttackIndicator`)
    (:`then`
      (`self.SetActorHiddenInGame` _attackindicator SetHidden)
      (bind _output_get (set `self.ActualAttackLocation` (+ LocationOffsetFromPlayer (`self.Attack Position`))))
      (`self.K2_SetActorLocation` _attackindicator _output_get false false))
    (:`else`)))

(fn `LerpOpacity`
  (for _array_element (`self.DynamicVanishMaterials`)
    (`MaterialInstanceDynamic.SetScalarParameterValue` _array_element "Opacity" 0.4))
  (set `self.OpacityValue` (`KismetMathLibrary.FInterpTo` (`self.OpacityValue`) 0.0 (`GameplayStatics.GetWorldDeltaSeconds`) (`self.VanishSpeed`))))

(fn `LoseLimb`
  (params (IsLeftLimb :type Boolean))
  (locals (LeftLimbWasLost :type Boolean))
  (bind _boss (`self.Boss`))
  (bind _armname (`self.GetArmName` (`local.LeftLimbWasLost`) true))
  (bind _output_get (set `local.LeftLimbWasLost` IsLeftLimb))
  (if _output_get
    (set `self.LostLeftLimb` true)
    (else
      (set `self.LostRightLimb` true)))
  (`SkeletalMeshComponent.SetAllBodiesBelowSimulatePhysics` _boss _armname true true)
  (`SkeletalMeshComponent.BreakConstraint` _boss (0.0 0.0 0.0) (`self.K2_GetActorLocation`) _armname)
  (`SkeletalMeshComponent.SetBodyNotifyRigidBodyCollision` _boss false _armname)
  (`self.Make Lost Limb Disappear` _armname)
  (`PrimitiveComponent.SetCollisionEnabled` (select `bool` (`local.LeftLimbWasLost`) :`false` (`self.RightLegUp`) :`true` (`self.LeftLegUp`) :!type "PrimitiveComponent Object Reference") "NoCollision")
  (`PrimitiveComponent.SetCollisionEnabled` (select `bool` (`local.LeftLimbWasLost`) :`false` (`self.RightLegDown`) :`true` (`self.LeftLegDown`)) "NoCollision")
  (if (`self.LostBothLimbs`)
    (`self.Die`)))

(fn `LostBothLimbs`
  (returns (ReturnValue :type Boolean))
  (return (and (`self.LostLeftLimb`) (`self.LostRightLimb`))))

(fn `PlayBoulderSequence`
  (bind _bossdamagedsequenceactor (`self.BossDamagedSequenceActor`)
    (:`then`
      (`MovieSceneSequencePlayer.Play` (`LevelSequenceActor.SequencePlayer` _bossdamagedsequenceactor))
      (bind _finalrock (`self.FinalRock`)
        (:`then`
          (`/Game/SimonStuff/Stuff/BP_BigRockBossKillah.Activate` _finalrock))
        (:`else`)))
    (:`else`)))

(fn `SetDestuctibleInMouth`
  (bind _returnvalue (`|SpawnActorFromClass` "/Game/_Game/Blueprints/Actors/BP_Destructable.BP_Destructable_C" (`KismetMathLibrary.MakeTransform` (`SceneComponent.K2_GetComponentLocation` (`self.LastHitEggLocation`))) "Undefined" "OverrideRootScale" null null))
  (set `/Game/_Game/Blueprints/Actors/BP_Destructable.AmountOfEnemiesToSpawnUponDestroyed` -1 _returnvalue)
  (`self.K2_AttachToComponent` _returnvalue (`self.Boss`) "MouthSocket" "KeepWorld" "KeepWorld" "KeepWorld" true)
  (add `/Game/_Game/Blueprints/Actors/BP_Destructable.TheEggExploded` _returnvalue (`|CreateDelegate` :!event `DissolveThisActor`)))

(fn `ShowLeftLegWeakPoints`
  (`self.ToggleWeakPoints` true false true)
  (`self.SpawnDirectionParticles` (`self.RightSigil`)))

(fn `ShowRightLegWeakPoints`
  (`self.ToggleWeakPoints` true true)
  (`self.SpawnDirectionParticles` (`self.LeftSigil`) (0.0 0.0 30.0) true))

(fn `SpawnAttackIndicator`
  (bind _returnvalue (`|SpawnActorFromClass` (`self.AttackIndicatorClass`) (`KismetMathLibrary.MakeTransform` (0.0 0.0 0.0) (struct) (3.0 3.0 3.0)) "Undefined" "OverrideRootScale" null null))
  (bind _output_get (set `self.AttackIndicator` _returnvalue))
  (`self.SetActorHiddenInGame` _output_get true))

(fn `SpawnDirectionParticles`
  (params (Sigil :type "/Game/SimonStuff/art/paintminigame/BP_PaintBoard Object Reference") (ParticleSpawnOffset :type "Vector Structure" :default (0.0 0.0 30.0)) (FromLeftSigil :type Boolean))
  (for _array_element (`self.AllWeakPoints`)
    (`/Engine/EditorBlueprintResources/StandardMacros.IsValid` _array_element
      (:`Is Valid`
        (if (not (== (`/Game/_Game/Blueprints/Components/Collisions/BP_HittableSphere.IsOnLeftSide` _array_element) FromLeftSigil))
          (bind _returnvalue (`NiagaraFunctionLibrary.SpawnSystemAtLocation` "/Game/_Game/VFX/VFX_MagicMissiles.VFX_MagicMissiles" (+ (`self.K2_GetActorLocation` Sigil) ParticleSpawnOffset)))
          (`FXSystemComponent.SetVectorParameter` _returnvalue "Target Position" (`SceneComponent.K2_GetComponentLocation` _array_element)))))))

(fn `Subscribe to Leg Weak Points`
  (locals (ArrayElementSphere :type "/Game/_Game/Blueprints/Components/Collisions/BP_HittableSphere Object Reference"))
  (bind _output_get (set `self.AllWeakPoints` (`|MakeArray` (`self.LeftLegWeakPoint1`) (`self.LeftLegWeakPoint2`) (`self.LeftLegWeakPoint3`) (`self.RightLegWeakPoint4`) (`self.RightLegWeakPoint5`) (`self.RightLegWeakPoint6`))))
  (for _array_element _output_get
    (set `local.ArrayElementSphere` _array_element)
    (if (`/Game/_Game/Blueprints/Components/Collisions/BP_HittableSphere.IsOnLeftSide` _array_element)
      (add `/Game/_Game/Blueprints/Components/Collisions/BP_HittableSphere.SphereGotHIt` (`local.ArrayElementSphere`) (`|CreateDelegate` :!event `DestroyLeftWeakPoint`))
      (else
        (add `/Game/_Game/Blueprints/Components/Collisions/BP_HittableSphere.SphereGotHIt` (`local.ArrayElementSphere`) (`|CreateDelegate` :!event `DestroyRightWeakPoint`))))
    (`SceneComponent.K2_AttachToComponent` (`local.ArrayElementSphere`) (`self.Boss`) (`self.GetArmName` (`/Game/_Game/Blueprints/Components/Collisions/BP_HittableSphere.IsOnLeftSide` (`local.ArrayElementSphere`)) true) "KeepWorld" "KeepWorld" "KeepWorld" true)))

(fn `SummonSupport`
  (params (JustLostLeftLimb :type Boolean) (SpawnOnWeakPointDestroyed :type Boolean) (WeakPointLocation :type "Vector Structure"))
  (for _ (range 1 (+ (`self.AmountOfEnemiesToSpawnWhenLostLimp`) 1))
    (bind _returnvalue (`|SpawnActorFromClass` (`self.SupportEnemyClass`) (`KismetMathLibrary.MakeTransform` (`KismetMathLibrary.SelectVector` WeakPointLocation (+ (* (`KismetMathLibrary.RandomUnitVector`) 20.0) (`SceneComponent.GetSocketLocation` (`self.Boss`) (`self.GetArmName` JustLostLeftLimb true))) SpawnOnWeakPointDestroyed) (struct) (`self.SupportEnemyScale`)) "Undefined" "OverrideRootScale" null null))
    (`/Engine/EditorBlueprintResources/StandardMacros.IsValid` _returnvalue
      (:`Is Valid`
        (`/Game/_Game/Blueprints/Characters/Enemies/BP_EnemyBase.SetIsAggravated` _returnvalue true (`GameplayStatics.GetPlayerCharacter` 0))))))

(fn `ToggleWeakPoints`
  (params (TurnOn :type Boolean) (ToggleRightSide :type Boolean) (ToggleLeftSide :type Boolean))
  (locals (IsOn :type Boolean) (RightSideIsOn :type Boolean) (LeftSideIsOn :type Boolean))
  (set `local.RightSideIsOn` ToggleRightSide)
  (set `local.LeftSideIsOn` ToggleLeftSide)
  (set `local.IsOn` TurnOn)
  (for _array_element (`self.AllWeakPoints`)
    (`/Engine/EditorBlueprintResources/StandardMacros.IsValid` _array_element
      (:`Is Valid`
        (bind _isonleftside (`/Game/_Game/Blueprints/Components/Collisions/BP_HittableSphere.IsOnLeftSide` _array_element))
        (if (or (and (`local.RightSideIsOn`) (not _isonleftside)) (and _isonleftside (`local.LeftSideIsOn`)))
          (`PrimitiveComponent.SetCollisionEnabled` _array_element (select `bool` (`local.IsOn`) :`false` "NoCollision" :`true` "QueryAndPhysics" :!type "ECollisionEnabled Enum"))
          (`SceneComponent.SetHiddenInGame` _array_element (not (`local.IsOn`)) true)
          (`SceneComponent.SetHiddenInGame` _array_element true false))))))

(fn `UserConstructionScript`)