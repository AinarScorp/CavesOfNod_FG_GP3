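; Tutorial variant of the rifle enemy that triggers bayonet tutorial feedback when killed.
; On BeginPlay it runs the parent logic, then becomes aggravated against the player immediately.
; On death it runs the parent logic, plays the player HUD's DeadBayonetTutorialAnim and plays a 2D voice line.
; An unconnected chain that plays and then reverses the same animation never runs.
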(event `self.ReceiveBeginPlay`
  (`parent.ReceiveBeginPlay`)
  (`self.SetIsAggravated` true (`GameplayStatics.GetPlayerCharacter` 0)))

(event `self.OnDeath`
  (`parent.OnDeath`)
  (bind _returnvalue (`GameplayStatics.GetActorOfClass` "/Game/_Game/Blueprints/Characters/BP_FirstPersonCharacter.BP_FirstPersonCharacter_C"))
  (bind _hud (`/Game/_Game/Blueprints/Characters/BP_FirstPersonCharacter.HUD` _returnvalue))
  (`UserWidget.PlayAnimation` _hud (`/Game/_Game/UI/HUD/WBP_HUD.DeadBayonetTutorialAnim` _hud) 0.0 1 "Forward" 1.0 false)
  (`GameplayStatics.PlaySound2D` (`self.VoiceLine`) 1.0 1.0 0.0 null null))

(fn `UserConstructionScript`
  (`parent.UserConstructionScript`))