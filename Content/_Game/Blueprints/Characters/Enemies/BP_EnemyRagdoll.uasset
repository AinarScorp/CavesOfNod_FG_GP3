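; Pooled ragdoll corpse of a dead enemy that players can stab to refill the stabbing weapon's ammo, with a hit effect.
; Pool events toggle skeletal mesh physics, and spawning also teleports the actor and restarts the emissive change.
; A looping timer drives a dynamic material's emissive intensity, but its clear condition compares constants and never passes.
; A helper hides detached leg bones and terminates their physics bodies.
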(event `self.ReceiveBeginPlay`
  (`self.SetNewDynamicMaterial`)
  (`self.StartChangingEmission`))

(event `LerpThroughEmission`
  (`EinarLibrary.ModifyAlphaLerp` (`self.Alpha`) (* (`GameplayStatics.GetWorldDeltaSeconds`) 10.0))
  (`MaterialInstanceDynamic.SetScalarParameterValue` (`self.DynamicMaterial`) "Emissive Intensity" (`KismetMathLibrary.Lerp` 1.0 0.01 (`self.Alpha`)))
  (if (>= 0.0 1.0)
    (`KismetSystemLibrary.K2_ClearAndInvalidateTimerHandle` (`self.FadeColorTimer`))))

(event `self.ApplyStabbing`
  (params (StabWeapon :type "TP_WeaponComponent Object Reference"))
  (`TP_WeaponComponent.ModifyCurrentAmmo` StabWeapon (`KismetMathLibrary.Conv_IntToDouble` (`TP_WeaponComponent.GetAmmoRefillOnDeadEnemy` StabWeapon)))
  (`NiagaraFunctionLibrary.SpawnSystemAtLocation` "/Game/_Game/VFX/FX_Hit.FX_Hit" (`SceneComponent.K2_GetComponentLocation` (`self.Scene`)) (struct :`Pitch` 90.0) (0.25 0.25 0.25)))

(event `self.SpawnPoolableActor`
  (params (Transform :type "Transform Structure"))
  (`self.K2_SetActorTransform` Transform false true)
  (`self.StartChangingEmission`)
  (`PrimitiveComponent.SetSimulatePhysics` (`self.SkeletalMesh`) true))

(event `self.SpawnByTheObjectPooling`
  (`PrimitiveComponent.SetSimulatePhysics` (`self.SkeletalMesh`) false))

(event `self.SkeletalMesh.OnComponentSleep`
  (params (SleepingComponent :type "PrimitiveComponent Object Reference") (BoneName :type Name))
  (`KismetSystemLibrary.PrintString` "sleeep"))

(fn `GetActor`
  (returns (ReturnValue :type "Actor Object Reference"))
  (return self))

(fn `HideDetachedLegs`
  (params (BoneNames :type "Array of Name"))
  (for _array_element BoneNames
    (`SkinnedMeshComponent.HideBoneByName` (`self.SkeletalMesh`) _array_element "PBO_Term")))

(fn `IsLockableStab`
  (returns (ReturnValue :type Boolean))
  (return true))

(fn `IsOneTimeStab`
  (returns (ReturnValue :type Boolean))
  (return false))

(fn `SetNewDynamicMaterial`
  (bind _returnvalue (`PrimitiveComponent.CreateDynamicMaterialInstance` (`self.SkeletalMesh`) 0 (`PrimitiveComponent.GetMaterial` (`self.SkeletalMesh`) 0) "DeadMaterial"))
  (bind _output_get (set `self.DynamicMaterial` _returnvalue))
  (`PrimitiveComponent.SetMaterial` (`self.SkeletalMesh`) 0 _output_get))

(fn `StartChangingEmission`
  (bind _output_get (set `self.Alpha` 1.0))
  (`MaterialInstanceDynamic.SetScalarParameterValue` (`self.DynamicMaterial`) "Emissive Intensity" _output_get)
  (bind _returnvalue (`KismetSystemLibrary.K2_SetTimerDelegate` (`|CreateDelegate` :!event `LerpThroughEmission`) 0.1 true 0.0 0.001))
  (set `self.FadeColorTimer` _returnvalue))

(fn `UserConstructionScript`)