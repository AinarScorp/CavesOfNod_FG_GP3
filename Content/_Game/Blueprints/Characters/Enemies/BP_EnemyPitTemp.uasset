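; BP_EnemyPitTemp is a temporary enemy Blueprint, extending a parent enemy, that becomes aggravated at the player as soon as play begins.
; Its attack sets the player's movement velocity to the enemy's velocity plus a strong forward push, then calls Launch Character with zero velocity and no overrides.
; On death it runs the parent logic, prints a debug string and calls CallCheckKilled.
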(event `self.ReceiveBeginPlay`
  (`parent.ReceiveBeginPlay`)
  (`self.SetIsAggravated` true (`GameplayStatics.GetPlayerCharacter` 0)))

(event `self.OnDeath`
  (`parent.OnDeath`)
  (`KismetSystemLibrary.PrintString` "IDieTHANKyOUfOREVA")
  (`self.CheckKilled`))

(event `self.PerformAttack`
  (bind _returnvalue (`self.GetMovementComponent`))
  (bind _returnvalue_2 (`GameplayStatics.GetPlayerCharacter` 0))
  (bind _returnvalue_3 (`self.GetMovementComponent` _returnvalue_2))
  (`parent.PerformAttack`)
  (`/Engine/EditorBlueprintResources/StandardMacros.IsValid` _returnvalue_3
    (:`Is Valid`
      (set `MovementComponent.Velocity` (+ (`MovementComponent.Velocity` _returnvalue) (* (`SceneComponent.GetForwardVector` (`MovementComponent.UpdatedComponent` _returnvalue)) 3000.0)) _returnvalue_3)
      (`Character.LaunchCharacter` _returnvalue_2 (0.0 0.0 0.0) false false))))

(fn `UserConstructionScript`
  (`parent.UserConstructionScript`))