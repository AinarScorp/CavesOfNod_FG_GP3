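; Acid spitter enemy that fires a projectile at the player as its ranged attack.
; While aggravated, Tick line-traces from its nose to the player, flagging attack range only with clear sight and under a distance threshold.
; PerformAttack turns it toward the player within the plane of its own up vector, preserving its surface tilt.
; It then spawns a test projectile class at the projectile point, aimed from the nose at the player.
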(event `self.PerformAttack`
  (bind _returnvalue (`EinarLibrary.GetTargetDirectionProjectedOnActorsPlane` (`GameplayStatics.GetPlayerCharacter` 0) self))
  (`self.K2_SetActorRotation` (`KismetMathLibrary.MakeRotationFromAxes` _returnvalue (`KismetMathLibrary.Normal` (`KismetMathLibrary.Cross_VectorVector` (`self.GetActorUpVector`) _returnvalue)) (`self.GetActorUpVector`)))
  (`|SpawnActorFromClass` "/Game/_Game/Blueprints/Actors/BP_ProjectileTestEinar.BP_ProjectileTestEinar_C" (`KismetMathLibrary.MakeTransform` (`SceneComponent.K2_GetComponentLocation` (`self.ProjectilePoint`)) (`KismetMathLibrary.MakeRotFromXZ` (`KismetMathLibrary.GetDirectionUnitVector` (`self.GetNoseLocation`) (`self.K2_GetActorLocation` (`GameplayStatics.GetPlayerCharacter` 0))) (`KismetMathLibrary.Vector_Up`))) "Undefined" "OverrideRootScale" self self))

(event `self.ReceiveTick`
  (params (DeltaSeconds :type "Float (single-precision)"))
  (if (`self.IsAggravatedToPlayer`)
    (bind (_outhit _returnvalue) (`KismetSystemLibrary.LineTraceSingle` (`self.GetNoseLocation`) (`self.K2_GetActorLocation` (`GameplayStatics.GetPlayerCharacter` 0)) "TraceTypeQuery5"))
    (if (and _returnvalue (== (`.HitActor` (`GameplayStatics.BreakHitResult` _outhit)) (`GameplayStatics.GetPlayerCharacter` 0)))
      (if (< (`.Distance` (`GameplayStatics.BreakHitResult` _outhit)) 1000.0)
        (`self.SetIsWithinAttackRange` true)
        (else
          (`self.SetIsWithinAttackRange` false :!label _label)))
      (else
        (goto _label)))))

(fn `UserConstructionScript`
  (`parent.UserConstructionScript`))