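; BP_BabyBugs is an enemy character Blueprint for baby bugs that are cleared from the level when a linked sigil completes.
; On BeginPlay it binds to the completion event of the sigil in SigilThatRemovesThese, if one is set.
; Completion triggers a configurable delay, then destroys the SpiderController, if valid, and the bug itself.
; Its PawnSensing see-pawn event is empty, so this graph adds no reaction to sighted pawns.
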(event `self.ReceiveBeginPlay`
  (`parent.ReceiveBeginPlay`)
  (bind _sigilthatremovesthese (`self.SigilThatRemovesThese`)
    (:`then`
      (add `/Game/SimonStuff/art/paintminigame/BP_PaintBoard.Sigil Complete` _sigilthatremovesthese (delegate `DestroyAfterDelay`)))
    (:`else`)))

(event `DestroyAfterDelay`
  (`KismetSystemLibrary.Delay` (`self.DeathDelay`))
  (bind _spidercontroller (`self.SpiderController`)
    (:`then`
      (`self.K2_DestroyActor` _spidercontroller))
    (:`else`
      _))
  (`self.K2_DestroyActor`))

(event `self.PawnSensing.OnSeePawn`
  (params (Pawn :type "Pawn Object Reference")))

(fn `UserConstructionScript`
  (`parent.UserConstructionScript`))