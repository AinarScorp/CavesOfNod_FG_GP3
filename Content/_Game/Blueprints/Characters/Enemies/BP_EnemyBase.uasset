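; Base spider-like enemy pawn that moves with path tracing and custom gravity, pulling itself to the ground when idle.
; It starts a behaviour tree on its controller and feeds sight, damage and attack-range events into the blackboard.
; Attacks damage the player directly, and death swaps in a pooled ragdoll.
; Personal-space collision switches off temporarily when blocked away from the player; limb detaching, montage playback and obstacle avoidance are unconnected.
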(event `self.ReceiveBeginPlay`
  (set `self.Tags` (`|MakeArray` (`self.Enemy`)))
  ;[0.1775 0.1653 1] Bind To events
  (add `HealthComponent.OnDie` (`self.HealthComponent`) (`|CreateDelegate` :!event `OnDeath`))
  (add `self.OnTakeAnyDamage` (`|CreateDelegate` :!event `Event On Take Damage`))
  (`self.Setup Controller and RunBehaviourTree`)
  (`self.PullToTheGround`)
  (bind _asbp_first_person_game_mode (cast `/Game/_Game/Blueprints/BP_FirstPersonGameMode` (`GameplayStatics.GetGameMode`)))
  (set `self.FP_GameModeCached` _asbp_first_person_game_mode))

(event `self.ToggleMovement`
  (params (TurnOn :type Boolean) (TargetRotation :type "Rotator Structure") (ChangeAlphaMultiplier :type "Float (single-precision)"))
  (`PathTracer.ToggleTracing` (`self.PathTracer`) TurnOn)
  (if TurnOn
    (`self.SetTargetToRotateTo` TargetRotation ChangeAlphaMultiplier)
    (`self.StartPlayingMoveSound`)
    (`self.PullToTheGround`)
    (else
      (`self.StopPlayingMoveSound`))))

(event `self.Move`
  (`parent.Move`)
  (`self.RotateToTarget`)
  (`self.IsMoving`
    (:`Yes`
      (`self.AddMovementInputToTargetLocation`)
      (`self.AlignRotation`))
    (:`No`
      (`self.PullToTheGround`))))

(event `self.PerformAttack`
  (`parent.PerformAttack`) ; I don't do anything
  ;[0.09783 1 0.1892] This should be triggered by animation inside anim montage
  (`GameplayStatics.ApplyDamage` (`GameplayStatics.GetPlayerCharacter` 0) (`self.Base Damage`)))

(event `Event On Take Damage` :!signature `self.OnTakeAnyDamage`
  (params (DamagedActor :type "Actor Object Reference") (Damage :type "Float (single-precision)") (DamageType :type "DamageType Object Reference") (InstigatedBy :type "Controller Object Reference") (DamageCauser :type "Actor Object Reference"))
  (`HealthComponent.TakeDamage` (`self.HealthComponent`) (`KismetMathLibrary.FTrunc` Damage))
  (`self.SetIsAggravated` true DamageCauser)
  (`GameplayStatics.PlaySoundAtLocation` "/Game/_Game/Sounds/MetaSounds/SFX_EnemyDamaged.SFX_EnemyDamaged" (`self.K2_GetActorLocation`) (struct) 1.0 1.0 0.0 null null null null)
  (`self.DetachLimb`))

(event `OnDeath`
  (`self.K2_DestroyActor` (`self.SpiderController`))
  (bind _returnvalue (`self.ReplaceThisActorWithRagdoll`))
  (`GameplayStatics.PlaySoundAtLocation` "/Game/_Game/Sounds/MetaSounds/SFX_EnemyDeath.SFX_EnemyDeath" _returnvalue (struct) 1.0 1.0 0.0 null null null null)
  (`self.SetActorHiddenInGame` self true)
  (`KismetSystemLibrary.Delay` 0.1)
  (`self.K2_DestroyActor`))

(event `self.AttackRange.OnComponentBeginOverlap`
  (params (OverlappedComponent :type "PrimitiveComponent Object Reference") (OtherActor :type "Actor Object Reference") (OtherComp :type "PrimitiveComponent Object Reference") (OtherBodyIndex :type Integer) (bFromSweep :type Boolean) (SweepResult :type "HitResult Structure (by ref)"))
  (bind _returnvalue (`GameplayStatics.GetPlayerCharacter` 0))
  ;[1 0.006541 0] IsWithinAttackRange
  (if (== OtherActor _returnvalue)
    (`self.SetPlayerTarget` _returnvalue)
    (`self.SetIsWithinAttackRange` true)))

(event `self.AttackRange.OnComponentEndOverlap`
  (params (OverlappedComponent :type "PrimitiveComponent Object Reference") (OtherActor :type "Actor Object Reference") (OtherComp :type "PrimitiveComponent Object Reference") (OtherBodyIndex :type Integer))
  (bind _returnvalue (`GameplayStatics.GetPlayerCharacter` 0))
  ;[1 0.006541 0] IsWithinAttackRange
  (if (== OtherActor _returnvalue)
    (`self.SetPlayerTarget` _returnvalue)
    (`self.SetIsWithinAttackRange` false)))

(event `self.PawnSensing.OnSeePawn`
  (params (Pawn :type "Pawn Object Reference"))
  (bind _returnvalue (`GameplayStatics.GetPlayerCharacter` 0))
  (if (and (not (`self.IsAggravatedToPlayer`)) (== Pawn _returnvalue))
    (`self.SetIsAggravated` true _returnvalue)
    (set `self.IsAggravatedToPlayer` true)))

(event `self.PersonalSpace.OnComponentHit`
  (params (HitComponent :type "PrimitiveComponent Object Reference") (OtherActor :type "Actor Object Reference") (OtherComp :type "PrimitiveComponent Object Reference") (NormalImpulse :type "Vector Structure") (Hit :type "HitResult Structure (by ref)"))
  (if (and (not (`KismetSystemLibrary.K2_IsValidTimerHandle` (`self.PeronalSpaceChechTImer`))) (`self.NotCloseEnoughTothePlayer`))
    (`PrimitiveComponent.SetCollisionResponseToChannel` (`self.PersonalSpace`) "ECC_GameTraceChannel3" "ECR_Ignore")
    (bind _returnvalue (`KismetSystemLibrary.K2_SetTimerDelegate` (`|CreateDelegate` :!event `EnablePersonalSpace`) 1.0 true))
    (set `self.PeronalSpaceChechTImer` _returnvalue)))

(event `self.ApplyStabbing`
  (params (StabWeapon :type "TP_WeaponComponent Object Reference"))
  (`parent.ApplyStabbing` StabWeapon)
  (`NiagaraFunctionLibrary.SpawnSystemAtLocation` "/Game/_Game/VFX/FX_Hit.FX_Hit" (`self.K2_GetActorLocation`)))

(event `self.GetHit`
  (params (DamageAmount :type "Float (single-precision)") (EventInstigator :type "Controller Object Reference") (DamageCauser :type "Actor Object Reference") (Hit :type "HitResult Structure (by ref)"))
  (bind (_bblockinghit _binitialoverlap _time _distance _location _impactpoint _normal _impactnormal) (`GameplayStatics.BreakHitResult` Hit))
  (`parent.GetHit` DamageAmount EventInstigator DamageCauser Hit)
  (`NiagaraFunctionLibrary.SpawnSystemAtLocation` "/Game/_Game/VFX/FX_Hit.FX_Hit" _impactpoint (`KismetMathLibrary.MakeRotFromX` _impactnormal) (0.3 0.3 0.3)))

(event `/Game/_Game/Interfaces/BPI_BossHittable.GetHitByBoss`
  (params (BossActor :type "Actor Object Reference"))
  (`GameplayStatics.ApplyDamage` self 99999.0 null BossActor))

(fn `DetachLimb`
  (bind _returnvalue (`HealthComponent.GetHealthPercent` (`self.HealthComponent`)))
  (if (>= (- (`self.LoseLimpTreshold`) _returnvalue) 0.25)
    (set `self.LoseLimpTreshold` _returnvalue)))

(fn `EnablePersonalSpace`
  (locals (SphereTrace :type "Array of EObjectTypeQuery Enum"))
  (bind _personalspace (`self.PersonalSpace`))
  (if (not (`self.NotCloseEnoughTothePlayer`))
    (`PrimitiveComponent.SetCollisionResponseToChannel` _personalspace "ECC_GameTraceChannel3" "ECR_Block" :!label _label)
    (`CapsuleComponent.SetCapsuleHalfHeight` _personalspace (`CapsuleComponent.CapsuleHalfHeight` _personalspace) true)
    (`KismetSystemLibrary.K2_ClearAndInvalidateTimerHandle` (`self.PeronalSpaceChechTImer`))
    (else
      (bind (_outhit _returnvalue) (`KismetSystemLibrary.SphereTraceSingleForObjects` (`self.K2_GetActorLocation`) (+ (`self.K2_GetActorLocation`) (* (`self.GetActorForwardVector`) 1.0)) (+ (`SphereComponent.GetScaledSphereRadius` (`self.Sphere`)) 0.0) (`local.SphereTrace`)))
      (if (not _returnvalue)
        (goto _label)))))

(fn `GetNoseLocation`
  (returns (NoseLocation :type "Vector Structure"))
  (return (`SceneComponent.K2_GetComponentLocation` (`self.NosePoint`))))

(fn `NotCloseEnoughTothePlayer`
  (returns (ReturnValue :type Boolean))
  (return (> (`KismetMathLibrary.Vector_Distance` (`self.K2_GetActorLocation` (`GameplayStatics.GetPlayerCharacter` 0)) (`self.K2_GetActorLocation`)) (`self.DistanceToPlayerForPersonalSpace`))))

(fn `PlaySoundInterval`
  (`GameplayStatics.PlaySoundAtLocation` (`self.EnemyFootStep`) (`self.K2_GetActorLocation`) (struct) 1.0 1.0 0.0 null null null null))

(fn `PullToTheGround`
  (bind _customgravity (`self.CustomGravity`))
  (if (not (`KismetSystemLibrary.K2_IsTimerActiveHandle` (`self.PullingToGroundTImer`)))
    (`CustomGravity.IsGrounded` _customgravity
      (:`Yes`
        (`self.StopPullingToTheGroundIfGrounded`))
      (:`No`
        (`CustomGravity.SetUseGravity` _customgravity true)
        (bind _returnvalue (`KismetSystemLibrary.K2_SetTimerDelegate` (`|CreateDelegate` :!event `StopPullingToTheGroundIfGrounded`) 0.1 true))
        (set `self.PullingToGroundTImer` _returnvalue)))))

(fn `ReplaceThisActorWithRagdoll`
  (returns (ReturnValue :type "Vector Structure"))
  (bind _returnvalue (`ActorPool.GetPooledActor` (`/Game/_Game/Blueprints/BP_FirstPersonGameMode.RagdollEnemyPool` (`self.FP_GameModeCached`))))
  (`PoolabelActor.SpawnPoolableActor` _returnvalue (`SceneComponent.K2_GetComponentToWorld` (`self.SkeletalMesh`)))
  (bind _returnvalue_2 (`PoolabelActor.GetActor` _returnvalue))
  (bind _asbp_enemy_ragdoll (cast `/Game/_Game/Blueprints/Characters/Enemies/BP_EnemyRagdoll` _returnvalue_2)
    (:`then`
      (`/Game/_Game/Blueprints/Characters/Enemies/BP_EnemyRagdoll.HideDetachedLegs` _asbp_enemy_ragdoll (`self.DetachedLimbesNames`)))
    (:`CastFailed`
      _))
  (return (`self.K2_GetActorLocation`)))

(fn `SetEmergencyFall`
  (params (Value :type Boolean))
  (`self.StopPullingToTheGroundIfGrounded`)
  (bind _spidercontroller (`self.SpiderController`)
    (:`then`
      (`/Game/_Game/Blueprints/Controllers/BP_EnemyControllerBase.SetBlackBoardBool` _spidercontroller "NewEnumerator2" Value))
    (:`else`)))

(fn `SetIsAggravated`
  (params (IsAggravated :type Boolean) (Aggravator :type "Actor Object Reference"))
  (bind _spidercontroller (`self.SpiderController`)
    (:`then`
      (`/Game/_Game/Blueprints/Controllers/BP_EnemyControllerBase.SetBlackBoardBool` _spidercontroller "NewEnumerator0" IsAggravated)
      (if IsAggravated
        (`self.SetPlayerTarget` Aggravator)))
    (:`else`)))

(fn `SetIsWithinAttackRange`
  (params (IsWithinAttackRange :type Boolean))
  (bind _spidercontroller (`self.SpiderController`)
    (:`then`
      (`/Game/_Game/Blueprints/Controllers/BP_EnemyControllerBase.SetBlackBoardBool` _spidercontroller "NewEnumerator1" IsWithinAttackRange))
    (:`else`)))

(fn `SetPlayerTarget`
  (params (AttackTarget :type "Actor Object Reference"))
  (bind _spidercontroller (`self.SpiderController`)
    (:`then`
      (`/Game/_Game/Blueprints/Controllers/BP_EnemyControllerBase.SetBlackboardObject` _spidercontroller "NewEnumerator1" AttackTarget))
    (:`else`)))

(fn `Setup Controller and RunBehaviourTree`
  (bind _asbp_enemy_controller_base (cast `/Game/_Game/Blueprints/Controllers/BP_EnemyControllerBase` (`self.GetController`)))
  (bind _output_get (set `self.SpiderController` _asbp_enemy_controller_base))
  (`/Game/_Game/Blueprints/Controllers/BP_EnemyControllerBase.SetStartingValues` _output_get (`self.ShouldWander`) (`self.WanderDurationMax`) (`self.WanderDurationMin`) (`self.CanDropOnTarget`) (`self.AcceptanceLengthForDrop`))
  (`AIController.RunBehaviorTree` (`self.SpiderController`) (`self.BehaviorTree`)))

(fn `StartPlayingMoveSound`
  (bind _returnvalue (`KismetSystemLibrary.K2_SetTimerDelegate` (`|CreateDelegate` :!event `PlaySoundInterval`) 0.5 true))
  (set `self.SoundLoopTimer` _returnvalue))

(fn `StopPlayingMoveSound`
  (`KismetSystemLibrary.K2_ClearAndInvalidateTimerHandle` (`self.SoundLoopTimer`)))

(fn `StopPullingToTheGroundIfGrounded`
  (bind _customgravity (`self.CustomGravity`))
  (`CustomGravity.IsGrounded` _customgravity
    (:`Yes`
      (`CustomGravity.SetUseGravity` _customgravity false)
      (`KismetSystemLibrary.K2_ClearAndInvalidateTimerHandle` (`self.PullingToGroundTImer`)))))

(fn `UserConstructionScript`)