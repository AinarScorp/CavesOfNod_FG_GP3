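; BP_Checkpoint is a checkpoint altar actor that lights up when the first-person character reaches it.
; BeginPlay creates a dynamic material instance on the altar mesh and zeroes its emissive parameter.
; A collision overlap sets the emissive to full and disables the collision when the actor is BP_FirstPersonCharacter.
; DoOnce runs before that cast, so any first overlap consumes it, and no respawn or save logic is present.
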(event `self.ReceiveBeginPlay`
  (bind _returnvalue (`PrimitiveComponent.CreateDynamicMaterialInstance` (`self.SM_Checkpoint_Altar`) 1 null (`self.EmissiveParameter`)))
  (bind _output_get (set `self.Material` _returnvalue))
  (`MaterialInstanceDynamic.SetScalarParameterValue` _output_get (`self.EmissiveParameter`) 0.0))

(event `self.CollisionComponent.OnComponentBeginOverlap`
  (params (OverlappedComponent :type "PrimitiveComponent Object Reference") (OtherActor :type "Actor Object Reference") (OtherComp :type "PrimitiveComponent Object Reference") (OtherBodyIndex :type Integer) (bFromSweep :type Boolean) (SweepResult :type "HitResult Structure (by ref)"))
  (`/Engine/EditorBlueprintResources/StandardMacros.DoOnce` false
    (:`Completed`
      (cast `/Game/_Game/Blueprints/Characters/BP_FirstPersonCharacter` OtherActor)
      (`MaterialInstanceDynamic.SetScalarParameterValue` (`self.Material`) (`self.EmissiveParameter`) 1.0)
      (`PrimitiveComponent.SetCollisionEnabled` (`self.CollisionComponent`) "NoCollision"))))

(fn `UserConstructionScript`)