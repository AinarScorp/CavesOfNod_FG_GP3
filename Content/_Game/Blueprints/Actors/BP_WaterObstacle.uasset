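; BP_WaterObstacle is a water hazard actor that damages the first-person player character over time while it is inside the Box volume.
; BeginPlay caches the player character as the damage target.
; A player overlap starts a looping one-second timer, apparently bound to DealDamage, which applies fixed damage to that cached character.
; Ending the overlap clears the timer, stopping further damage.
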(event `self.ReceiveBeginPlay`
  (bind _asbp_first_person_character (cast `/Game/_Game/Blueprints/Characters/BP_FirstPersonCharacter` (`GameplayStatics.GetPlayerCharacter` 0)))
  (set `self.As BP First Person Character` _asbp_first_person_character))

(event `DealDamage`
  ;[1 1 1] DealDamageEvent
  (`GameplayStatics.ApplyDamage` (`self.As BP First Person Character`) 10.0))

(event `self.Box.OnComponentBeginOverlap`
  (params (OverlappedComponent :type "PrimitiveComponent Object Reference") (OtherActor :type "Actor Object Reference") (OtherComp :type "PrimitiveComponent Object Reference") (OtherBodyIndex :type Integer) (bFromSweep :type Boolean) (SweepResult :type "HitResult Structure (by ref)"))
  ;[1 1 1] Deals damage to the player
  (cast `/Game/_Game/Blueprints/Characters/BP_FirstPersonCharacter` OtherActor)
  (bind _returnvalue (`KismetSystemLibrary.K2_SetTimerDelegate` (`|CreateDelegate` :!event `DealDamage`) 1.0 true)))

(event `self.Box.OnComponentEndOverlap`
  (params (OverlappedComponent :type "PrimitiveComponent Object Reference") (OtherActor :type "Actor Object Reference") (OtherComp :type "PrimitiveComponent Object Reference") (OtherBodyIndex :type Integer))
  ;[1 1 1] Stops Dealing Damage
  (cast `/Game/_Game/Blueprints/Characters/BP_FirstPersonCharacter` OtherActor)
  (`KismetSystemLibrary.K2_ClearAndInvalidateTimerHandle` (stale `self.Box.OnComponentBeginOverlap` _returnvalue)))

(fn `UserConstructionScript`)