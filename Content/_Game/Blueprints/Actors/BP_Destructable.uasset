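; BP_Destructable is a destructible egg actor that releases enemies when it explodes.
; Its Explode event runs SpawnEnemiesFromTheEgg, then destroys the actor.
; That function spawns a configurable number of BP_EnemyBase at small random offsets around the egg, aggravates each against player character 0, then calls TheEggExploded.
; Leftover nodes for an Eggsplosive cast and a direct Explode call are never run.
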(event `self.Explode`
  (params (DamageAmount :type "Float (single-precision)") (EventInstigator :type "Controller Object Reference") (DamageCauser :type "Actor Object Reference"))
  (`self.SpawnEnemiesFromTheEgg`)
  (`self.K2_DestroyActor`))

(fn `SpawnEnemiesFromTheEgg`
  (for _ (range 1 (+ (`self.AmountOfEnemiesToSpawnUponDestroyed`) 1))
    (bind _returnvalue (`|SpawnActorFromClass` "/Game/_Game/Blueprints/Characters/Enemies/BP_EnemyBase.BP_EnemyBase_C" (`KismetMathLibrary.MakeTransform` (+ (* (`KismetMathLibrary.RandomUnitVector`) 50.0) (`self.K2_GetActorLocation`))) "AdjustIfPossibleButAlwaysSpawn" "OverrideRootScale" null null))
    (`/Engine/EditorBlueprintResources/StandardMacros.IsValid` _returnvalue
      (:`Is Valid`
        (`/Game/_Game/Blueprints/Characters/Enemies/BP_EnemyBase.SetIsAggravated` _returnvalue true (`GameplayStatics.GetPlayerCharacter` 0)))))
  (`self.TheEggExploded`))

(fn `UserConstructionScript`)