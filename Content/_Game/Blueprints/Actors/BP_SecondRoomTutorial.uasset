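; BP_SecondRoomTutorial is a one-shot trigger box that shows the second room tutorial on the first-person character's HUD.
; Begin overlap reverses the dead bayonet tutorial animation, waits briefly, then plays the second room animation.
; End overlap reverses that animation and destroys the actor.
; Each DoOnce precedes the character cast, so any overlapping actor can use it up.
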(event `self.Box.OnComponentBeginOverlap`
  (params (OverlappedComponent :type "PrimitiveComponent Object Reference") (OtherActor :type "Actor Object Reference") (OtherComp :type "PrimitiveComponent Object Reference") (OtherBodyIndex :type Integer) (bFromSweep :type Boolean) (SweepResult :type "HitResult Structure (by ref)"))
  (`/Engine/EditorBlueprintResources/StandardMacros.DoOnce` false
    (:`Completed`
      (bind _asbp_first_person_character (cast `/Game/_Game/Blueprints/Characters/BP_FirstPersonCharacter` OtherActor))
      (bind _hud (`/Game/_Game/Blueprints/Characters/BP_FirstPersonCharacter.HUD` _asbp_first_person_character))
      (`UserWidget.PlayAnimationReverse` _hud (`/Game/_Game/UI/HUD/WBP_HUD.DeadBayonetTutorialAnim` _hud) 1.0 false)
      (`KismetSystemLibrary.Delay` 2.0)
      (`UserWidget.PlayAnimation` _hud (`/Game/_Game/UI/HUD/WBP_HUD.SecondRoomTutorialAnim` _hud) 0.0 1 "Forward" 1.0 false))))

(event `self.Box.OnComponentEndOverlap`
  (params (OverlappedComponent :type "PrimitiveComponent Object Reference") (OtherActor :type "Actor Object Reference") (OtherComp :type "PrimitiveComponent Object Reference") (OtherBodyIndex :type Integer))
  (`/Engine/EditorBlueprintResources/StandardMacros.DoOnce` false
    (:`Completed`
      (cast `/Game/_Game/Blueprints/Characters/BP_FirstPersonCharacter` OtherActor)
      (bind _hud (`/Game/_Game/Blueprints/Characters/BP_FirstPersonCharacter.HUD` (stale `self.Box.OnComponentBeginOverlap` _asbp_first_person_character)))
      (`UserWidget.PlayAnimationReverse` _hud (`/Game/_Game/UI/HUD/WBP_HUD.SecondRoomTutorialAnim` _hud) 1.0 false)
      (`self.K2_DestroyActor`))))

(fn `UserConstructionScript`)