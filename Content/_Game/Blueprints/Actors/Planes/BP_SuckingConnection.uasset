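; BP_SuckingConnection is a plane actor that visually spans, by its name a suction link, between an origin component and a target point.
; PlaceConnection stores both ends and places the actor immediately.
; Tick repeats placement while the origin is valid, following the component toward the fixed target.
; Placement centers the actor at the midpoint, points X at the target and scales all axes uniformly by distance over 100.
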(event `self.ReceiveTick`
  (params (DeltaSeconds :type "Float (single-precision)"))
  (if (`KismetSystemLibrary.IsValid` (`self.OriginComponent`))
    (`self.PlaceActorInMiddle`)))

(fn `PlaceActorInMiddle`
  (bind _targetpoint (`self.TargetPoint`))
  (bind _returnvalue (`SceneComponent.K2_GetComponentLocation` (`self.OriginComponent`)))
  (bind _returnvalue_2 (- _targetpoint _returnvalue))
  (`self.K2_SetActorLocation` (`KismetMathLibrary.VLerp` _returnvalue _targetpoint 0.5))
  (`self.K2_SetActorRotation` (`KismetMathLibrary.MakeRotFromX` _returnvalue_2))
  (`self.SetActorScale3D` (`KismetMathLibrary.Conv_DoubleToVector` (/ (`KismetMathLibrary.VSize` _returnvalue_2) 100.0))))

(fn `PlaceConnection`
  (params (OriginComponent :type "SceneComponent Object Reference") (TargetPoint :type "Vector Structure"))
  (set `self.OriginComponent` OriginComponent)
  (set `self.TargetPoint` TargetPoint)
  (`self.PlaceActorInMiddle`))

(fn `UserConstructionScript`)