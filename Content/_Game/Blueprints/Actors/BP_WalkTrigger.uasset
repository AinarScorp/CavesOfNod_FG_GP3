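; BP_WalkTrigger is a trigger-box actor for a scripted jumpscare in which an enemy walks to a goal and disappears.
; When BP_FirstPersonCharacter overlaps the box, it sets Goal as the enemy's player target and starts a looping timer.
; DestroyOnDone removes both enemy and trigger once the enemy is close to the goal.
; On BeginPlay, the trigger destroys itself and prints a message if either reference is unset.
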(event `self.ReceiveBeginPlay`
  (`self.DestroysIfNotValid`))

(event `self.Box.OnComponentBeginOverlap`
  (params (OverlappedComponent :type "PrimitiveComponent Object Reference") (OtherActor :type "Actor Object Reference") (OtherComp :type "PrimitiveComponent Object Reference") (OtherBodyIndex :type Integer) (bFromSweep :type Boolean) (SweepResult :type "HitResult Structure (by ref)"))
  (cast `/Game/_Game/Blueprints/Characters/BP_FirstPersonCharacter` OtherActor)
  (`self.Jumpscare`))

(event `Jumpscare`
  (`/Game/_Game/Blueprints/Characters/Enemies/BP_EnemyBase.SetPlayerTarget` (`self.EnemyRef1`) (`self.Goal`))
  (`KismetSystemLibrary.K2_SetTimerDelegate` (`|CreateDelegate` :!event `DestroyOnDone`) 0.1 true))

(event `DestroyOnDone`
  (if (< (`self.GetDistanceTo` (`self.EnemyRef1`) (`self.Goal`)) 59.0)
    (`self.K2_DestroyActor` (`self.EnemyRef1`))
    (`self.K2_DestroyActor`)))

(fn `DestroysIfNotValid`
  (if (not (and (`KismetSystemLibrary.IsValid` (`self.Goal`)) (`KismetSystemLibrary.IsValid` (`self.EnemyRef1`))))
    (`self.K2_DestroyActor`)
    (`KismetSystemLibrary.PrintText` (`|FormatText` "I'm not set up{Name}" (`KismetSystemLibrary.GetDisplayName` self)))))

(fn `UserConstructionScript`)