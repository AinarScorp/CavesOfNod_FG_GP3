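; BP_FinalDoor is a door actor that slides open when its SpawnerBoss reference fires the bound open-door event.
; It stores its start location on BeginPlay and binds OpenDoor to that event.
; OpenDoor plays a timeline that lerps the door from its start location to an OpenPosition offset with sweep enabled.
; The door sound is triggered on every timeline update rather than once.
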(event `self.ReceiveBeginPlay`
  (set `self.StartPosition` (`self.K2_GetActorLocation`))
  (add `/Game/_Game/Blueprints/Actors/BP_BossSpawner.OpenDoor` (`self.SpawnerBoss`) (delegate `OpenDoor`)))

(event `OpenDoor`
  (bind _startposition (`self.StartPosition`))
  (bind (_direction _newtrack_0) (`Timeline|Timeline` :!via `PlayFromStart`)
    (:`Update`
      (`self.K2_SetActorLocation` (`KismetMathLibrary.VLerp` _startposition (+ _startposition (`self.OpenPosition`)) _newtrack_0) true)
      (`GameplayStatics.PlaySoundAtLocation` "/Game/_Game/Sounds/MetaSounds/SFX_DoorSound.SFX_DoorSound" (`self.K2_GetActorLocation`) (struct) 1.0 1.0 0.0 null null null null))))

(fn `UserConstructionScript`)