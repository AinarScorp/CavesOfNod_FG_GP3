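; Healing egg pickup that the player consumes by stabbing it, then respawns after a delay.
; A stab hides the egg, glow and light, spawns a splat effect, heals the player and plays the HUD heal animation.
; A timer restores the visuals and availability, and the stab queries report it as one-time and non-lockable.
; An interact-and-hover path granting health packs remains as disconnected logic.
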(event `self.Interact`)

(event `Respawn egg`
  (`KismetSystemLibrary.K2_ClearAndInvalidateTimerHandle` (`self.respawn timer object`))
  (`SceneComponent.SetVisibility` (`self.Glow`) true false)
  (`SceneComponent.SetVisibility` (`self.egg`) true false)
  (`SceneComponent.SetVisibility` (`self.PointLight`) true false)
  (set `self.hasEgg` true))

(event `self.BeginHover`)

(event `self.EndHover`)

(event `self.ApplyStabbing`
  (params (StabWeapon :type "TP_WeaponComponent Object Reference"))
  (bind _asbp_first_person_character (cast `/Game/_Game/Blueprints/Characters/BP_FirstPersonCharacter` (`GameplayStatics.GetPlayerPawn` 0) :!pure true))
  (bind _hud (`/Game/_Game/Blueprints/Characters/BP_FirstPersonCharacter.HUD` _asbp_first_person_character))
  (if (`self.hasEgg`)
    (bind _returnvalue (`KismetSystemLibrary.K2_SetTimerDelegate` (delegate `CustomEvent_2`) (`self.RespawnTimer`)))
    (set `self.respawn timer object` _returnvalue)
    (`SceneComponent.SetVisibility` (`self.egg`) false false)
    (`SceneComponent.SetVisibility` (`self.Glow`) false false)
    (`SceneComponent.SetVisibility` (`self.PointLight`) false false)
    (set `self.hasEgg` false)
    (`NiagaraFunctionLibrary.SpawnSystemAtLocation` "/Game/_Game/VFX/FX_HealingSplat.FX_HealingSplat" (`self.K2_GetActorLocation`))
    (`HealthComponent.Heal` (`TP_FirstPersonCharacter.Health` _asbp_first_person_character) 200)
    (`UserWidget.PlayAnimation` _hud (`/Game/_Game/UI/HUD/WBP_HUD.Heal` _hud) 0.0 1 "Forward" 1.0 false)))

(event `CustomEvent_2`
  (`KismetSystemLibrary.K2_ClearAndInvalidateTimerHandle` (`self.respawn timer object`))
  (`SceneComponent.SetVisibility` (`self.Glow`) true false)
  (`SceneComponent.SetVisibility` (`self.egg`) true false)
  (`SceneComponent.SetVisibility` (`self.PointLight`) true false)
  (set `self.hasEgg` true))

(event `CustomEvent_1`)

(event `CustomEvent`)

(event `CustomEvent_3`
  (params (StabWeapon :type "TP_WeaponComponent Object Reference")))

(fn `IsLockableStab`
  (returns (ReturnValue :type Boolean))
  (return false))

(fn `IsOneTimeStab`
  (returns (ReturnValue :type Boolean))
  (return true))

(fn `UserConstructionScript`)