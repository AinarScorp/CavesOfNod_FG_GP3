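; A test projectile that paints boards and spawns impact effects when it hits something, then destroys itself.
; OnHit runs the parent logic, then branches on the exact class of the hit actor.
; For BP_PaintBoard, a short trace through the impact point finds the collision UV, passed to DrawOnBoard, and spawns a splatter.
; BP_EnemyBase gets a hit effect aligned to the impact normal; anything else gets a splatter at the projectile's location.
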(event `self.OnHit`
  (params (HitComp :type "PrimitiveComponent Object Reference") (OtherActor :type "Actor Object Reference") (OtherComp :type "PrimitiveComponent Object Reference") (NormalImpulse :type "Vector Structure") (Hit :type "HitResult Structure (by ref)"))
  (bind (_bblockinghit _binitialoverlap _time _distance _location _impactpoint _normal _impactnormal) (`GameplayStatics.BreakHitResult` Hit))
  (bind _returnvalue (`GameplayStatics.GetObjectClass` OtherActor))
  (bind (_bblockinghit_2 _binitialoverlap_2 _time_2 _distance_2 _location_2 _impactpoint_2 _normal_2 _impactnormal_2) (`GameplayStatics.BreakHitResult` Hit))
  (`parent.OnHit` HitComp OtherActor OtherComp NormalImpulse Hit)
  (if (== _returnvalue "/Game/SimonStuff/art/paintminigame/BP_PaintBoard.BP_PaintBoard_C")
    (bind _outhit (`KismetSystemLibrary.LineTraceSingle` (+ _impactpoint_2 (* _impactnormal_2 10.0)) (+ _impactpoint_2 (* _impactnormal_2 -10.0)) "TraceTypeQuery1"))
    (bind (_bblockinghit_3 _binitialoverlap_3 _time_3 _distance_3 _location_3 _impactpoint_3 _normal_3 _impactnormal_3 _physmat _hitactor) (`GameplayStatics.BreakHitResult` _outhit))
    (`/Game/SimonStuff/art/paintminigame/BP_PaintBoard.DrawOnBoard` (cast `/Game/SimonStuff/art/paintminigame/BP_PaintBoard` _hitactor :!pure true) (`GameplayStatics.FindCollisionUV` _outhit))
    (`NiagaraFunctionLibrary.SpawnSystemAtLocation` "/Game/_Game/VFX/FX_Splatter.FX_Splatter" _location_3 (struct) (0.1 0.1 0.1))
    (elif (== _returnvalue "/Game/_Game/Blueprints/Characters/Enemies/BP_EnemyBase.BP_EnemyBase_C")
      (`NiagaraFunctionLibrary.SpawnSystemAtLocation` "/Game/_Game/VFX/FX_Hit.FX_Hit" _impactpoint (`KismetMathLibrary.MakeRotFromX` _impactnormal) (0.3 0.3 0.3))
      (else
        (`NiagaraFunctionLibrary.SpawnSystemAtLocation` "/Game/_Game/VFX/FX_Splatter.FX_Splatter" (`self.K2_GetActorLocation`) (struct) (0.1 0.1 0.1)))))
  (`self.K2_DestroyActor`))

(fn `UserConstructionScript`)