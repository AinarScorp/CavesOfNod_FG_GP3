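; Tutorial actor for room one that shows movement hints and scripts the loss of the player's pistol.
; Jump and long-jump trigger volumes play HUD tutorial animations when the player enters and reverse them on exit.
; DestroyPistol counts kills; from three onward it empties the pistol, plays timed dry-fire clicks, then hides it and the first-person mesh.
; Its binding to pistol enemies is disconnected, and the closing rifle lookup is unused.
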(event `self.ReceiveBeginPlay`)

(event `DestroyPistol`
  (bind _result (`/Engine/EditorBlueprintResources/StandardMacros.IncrementInt` (`self.KilledEnemies`))
    (:`  `
      (`/Engine/EditorBlueprintResources/StandardMacros.CompareInt` _result 3
        (:`>`
          _)
        (:`==`
          _))
      (bind _returnvalue (`GameplayStatics.GetActorOfClass` "/Game/_Game/Blueprints/Actors/BP_PickUp_Pistol.BP_PickUp_Pistol_C"))
      (bind _bp_pistol (`/Game/_Game/Blueprints/Actors/BP_PickUp_Pistol.BP_Pistol` _returnvalue))
      (set `TP_WeaponComponent.CurrentAmmo` 0 _bp_pistol)
      (`KismetSystemLibrary.Delay` 1.0)
      (`GameplayStatics.PlaySound2D` "/Game/_Game/Sounds/467183__sophia_c__pistol-dry-fire-bersa-bp9cc-9x19.467183__sophia_c__pistol-dry-fire-bersa-bp9cc-9x19" 1.0 1.0 0.0 null null)
      (`KismetSystemLibrary.Delay` 1.0)
      (`GameplayStatics.PlaySound2D` "/Game/_Game/Sounds/467183__sophia_c__pistol-dry-fire-bersa-bp9cc-9x19.467183__sophia_c__pistol-dry-fire-bersa-bp9cc-9x19" 1.0 1.0 0.0 null null)
      (`KismetSystemLibrary.Delay` 0.5)
      (`GameplayStatics.PlaySound2D` "/Game/_Game/Sounds/467183__sophia_c__pistol-dry-fire-bersa-bp9cc-9x19.467183__sophia_c__pistol-dry-fire-bersa-bp9cc-9x19" 1.0 1.0 0.0 null null)
      (`KismetSystemLibrary.Delay` 0.2)
      (`GameplayStatics.PlaySound2D` "/Game/_Game/Sounds/467183__sophia_c__pistol-dry-fire-bersa-bp9cc-9x19.467183__sophia_c__pistol-dry-fire-bersa-bp9cc-9x19" 1.0 1.0 0.0 null null)
      (`KismetSystemLibrary.Delay` 0.2)
      (`GameplayStatics.PlaySound2D` "/Game/_Game/Sounds/467183__sophia_c__pistol-dry-fire-bersa-bp9cc-9x19.467183__sophia_c__pistol-dry-fire-bersa-bp9cc-9x19" 1.0 1.0 0.0 null null)
      (`KismetSystemLibrary.Delay` 1.0)
      (`SceneComponent.SetVisibility` _bp_pistol false false)
      (bind _returnvalue_2 (`GameplayStatics.GetActorOfClass` "/Game/_Game/Blueprints/Characters/BP_FirstPersonCharacter.BP_FirstPersonCharacter_C"))
      (`SceneComponent.SetVisibility` (`TP_FirstPersonCharacter.Mesh1P` _returnvalue_2) false false)
      (`GameplayStatics.GetActorOfClass` "/Game/_Game/Blueprints/Actors/BP_PickUp_Rifle.BP_PickUp_Rifle_C"))))

(event `self.JumpCollider.OnComponentBeginOverlap`
  (params (OverlappedComponent :type "PrimitiveComponent Object Reference") (OtherActor :type "Actor Object Reference") (OtherComp :type "PrimitiveComponent Object Reference") (OtherBodyIndex :type Integer) (bFromSweep :type Boolean) (SweepResult :type "HitResult Structure (by ref)"))
  ;[1 1 1] Shows and hides tutorial for the jump
  (bind _asbp_first_person_character (cast `/Game/_Game/Blueprints/Characters/BP_FirstPersonCharacter` OtherActor))
  (bind _hud (`/Game/_Game/Blueprints/Characters/BP_FirstPersonCharacter.HUD` _asbp_first_person_character))
  (`UserWidget.PlayAnimation` _hud (`/Game/_Game/UI/HUD/WBP_HUD.JumpTutorialAnim` _hud) 0.0 1 "Forward" 1.0 false))

(event `self.JumpCollider.OnComponentEndOverlap`
  (params (OverlappedComponent :type "PrimitiveComponent Object Reference") (OtherActor :type "Actor Object Reference") (OtherComp :type "PrimitiveComponent Object Reference") (OtherBodyIndex :type Integer))
  ;[1 1 1] Shows and hides tutorial for the jump
  (bind _asbp_first_person_character (cast `/Game/_Game/Blueprints/Characters/BP_FirstPersonCharacter` OtherActor))
  (bind _hud (`/Game/_Game/Blueprints/Characters/BP_FirstPersonCharacter.HUD` _asbp_first_person_character))
  (`UserWidget.PlayAnimationReverse` _hud (`/Game/_Game/UI/HUD/WBP_HUD.JumpTutorialAnim` _hud) 1.0 false))

(event `self.LongJumpCollider.OnComponentBeginOverlap`
  (params (OverlappedComponent :type "PrimitiveComponent Object Reference") (OtherActor :type "Actor Object Reference") (OtherComp :type "PrimitiveComponent Object Reference") (OtherBodyIndex :type Integer) (bFromSweep :type Boolean) (SweepResult :type "HitResult Structure (by ref)"))
  ;[1 1 1] SHows and hides tutorial for long jump
  (bind _asbp_first_person_character (cast `/Game/_Game/Blueprints/Characters/BP_FirstPersonCharacter` OtherActor))
  (bind _hud (`/Game/_Game/Blueprints/Characters/BP_FirstPersonCharacter.HUD` _asbp_first_person_character))
  (`UserWidget.PlayAnimation` _hud (`/Game/_Game/UI/HUD/WBP_HUD.LongJumpTutorialAnim` _hud) 0.0 1 "Forward" 1.0 false))

(event `self.LongJumpCollider.OnComponentEndOverlap`
  (params (OverlappedComponent :type "PrimitiveComponent Object Reference") (OtherActor :type "Actor Object Reference") (OtherComp :type "PrimitiveComponent Object Reference") (OtherBodyIndex :type Integer))
  ;[1 1 1] SHows and hides tutorial for long jump
  (bind _asbp_first_person_character (cast `/Game/_Game/Blueprints/Characters/BP_FirstPersonCharacter` OtherActor))
  (bind _hud (`/Game/_Game/Blueprints/Characters/BP_FirstPersonCharacter.HUD` _asbp_first_person_character))
  (`UserWidget.PlayAnimationReverse` _hud (`/Game/_Game/UI/HUD/WBP_HUD.LongJumpTutorialAnim` _hud) 1.0 false))

(fn `UserConstructionScript`)