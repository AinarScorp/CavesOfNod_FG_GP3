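; BP_Eggsplosive is an explosive pickup that attaches to weapons and respawns at its starting location after exploding.
; It extends parent attach, stab and explode events, ignoring pawn and one custom collision channel once attached and removing its glow when stabbed.
; On explosion it plays effects and sound, hides its meshes, disables collision, then after a delay spawns a replacement and destroys itself.
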(event `self.ReceiveBeginPlay`
  (set `self.RespawnPoint` (`self.K2_GetActorLocation`)))

(event `self.AttachToWeapon`
  (params (Weapon :type "TP_WeaponComponent Object Reference"))
  (bind _collisioncomp (`self.CollisionComp`))
  (`parent.AttachToWeapon` Weapon)
  (`PrimitiveComponent.SetCollisionResponseToChannel` _collisioncomp "ECC_Pawn" "ECR_Ignore")
  (`PrimitiveComponent.SetCollisionResponseToChannel` _collisioncomp "ECC_GameTraceChannel1" "ECR_Ignore"))

(event `self.Eggsplode`
  (`parent.Eggsplode`)
  (`NiagaraFunctionLibrary.SpawnSystemAtLocation` "/Game/_Game/VFX/FX_Explotion.FX_Explotion" (`self.K2_GetActorLocation`))
  (`GameplayStatics.SpawnSoundAtLocation` "/Game/_Game/Sounds/MetaSounds/SFX_GrenadeBoom.SFX_GrenadeBoom" (`self.K2_GetActorLocation`) (struct) 1.0 1.0 0.0 null null)
  (`SceneComponent.SetVisibility` (`self.StaticMesh`) false false)
  (`SceneComponent.SetVisibility` (`self.StaticMesh1`) false false)
  (`PrimitiveComponent.SetCollisionResponseToAllChannels` (`self.CollisionComp`) "ECR_Ignore")
  (`KismetSystemLibrary.Delay` 10.0)
  (`|SpawnActorFromClass` "BP_Eggsplosive_C" (`KismetMathLibrary.Conv_VectorToTransform` (`self.RespawnPoint`)) "AlwaysSpawn" "OverrideRootScale" null null)
  (`self.K2_DestroyActor`))

(event `self.ApplyStabbing`
  (params (StabWeapon :type "TP_WeaponComponent Object Reference"))
  (`parent.ApplyStabbing` StabWeapon)
  (`ActorComponent.K2_DestroyComponent` (`self.Glow_2`)))

(fn `UserConstructionScript`)