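; BP_FinishGame is a trigger actor that plays the game's ending when the first-person character enters its box.
; On overlap it plays a voice line and the Ending level sequence while disabling player input.
; After a fixed delay it shows the cursor and finish credits widget, switches to UI-only input and hides the character's HUD.
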(event `self.Box.OnComponentBeginOverlap`
  (params (OverlappedComponent :type "PrimitiveComponent Object Reference") (OtherActor :type "Actor Object Reference") (OtherComp :type "PrimitiveComponent Object Reference") (OtherBodyIndex :type Integer) (bFromSweep :type Boolean) (SweepResult :type "HitResult Structure (by ref)"))
  (bind _returnvalue (`GameplayStatics.GetPlayerCharacter` 0))
  (bind _returnvalue_2 (`GameplayStatics.GetPlayerController` 0))
  (bind _asbp_first_person_character (cast `/Game/_Game/Blueprints/Characters/BP_FirstPersonCharacter` OtherActor))
  (set `self.CharacterRef` _asbp_first_person_character)
  (`GameplayStatics.PlaySound2D` (`self.VoiceLine`) 1.0 1.0 0.0 null null)
  (bind _outactor (`LevelSequencePlayer.CreateLevelSequencePlayer` "/Game/Ending.Ending"))
  (`MovieSceneSequencePlayer.Play` (`LevelSequenceActor.SequencePlayer` _outactor))
  (`self.DisableInput` _returnvalue _returnvalue_2)
  (`KismetSystemLibrary.Delay` 17.0)
  (set `PlayerController.bShowMouseCursor` true _returnvalue_2)
  (bind _returnvalue_3 (`|CreateWidget` "/Game/_Game/UI/WBP_FinishCredits.WBP_FinishCredits_C"))
  (`UserWidget.AddToViewport` _returnvalue_3 0)
  (`self.EnableInput` _returnvalue _returnvalue_2)
  (`WidgetBlueprintLibrary.SetInputMode_UIOnlyEx` _returnvalue_2 _returnvalue_3)
  (set `Widget.Visibility` "Hidden" (`/Game/_Game/Blueprints/Characters/BP_FirstPersonCharacter.HUD` (`self.CharacterRef`))))

(fn `UserConstructionScript`)