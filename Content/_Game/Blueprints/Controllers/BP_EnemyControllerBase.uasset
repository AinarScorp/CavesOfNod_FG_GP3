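; Base controller for enemy AI that provides helper functions for writing to the Blackboard.
; Typed setters for object, float and bool values derive each key name from an enum's string, so callers avoid raw key names.
; SetStartingValues uses the float and bool setters to seed wander settings (toggle, min and max duration) and drop-to-target settings (permission and acceptance length).
; The event graph holds no logic of its own.
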(event `self.ReceiveBeginPlay`)

(fn `SetBlackBoardBool`
  (params (`Bool Name` :type "/Game/_Game/EnemyBehaviours/Enums/BlackboardBoolNames Enum" :default "NewEnumerator0") (Value :type Boolean))
  (`BlackboardComponent.SetValueAsBool` (`self.BlackboardComponent`) (`KismetStringLibrary.Conv_StringToName` (`|GetEnumeratorNameAsString` `Bool Name`)) Value))

(fn `SetBlackBoardFloat`
  (params (`Bool Name` :type "/Game/_Game/EnemyBehaviours/Enums/BlackboardFloatNames Enum" :default "NewEnumerator0") (Value :type "Float (double-precision)"))
  (`BlackboardComponent.SetValueAsFloat` (`self.BlackboardComponent`) (`KismetStringLibrary.Conv_StringToName` (`|GetEnumeratorNameAsString` `Bool Name`)) Value))

(fn `SetBlackboardObject`
  (params (`ObjectType Name` :type "/Game/_Game/EnemyBehaviours/Enums/BlackboardObjectStrings Enum" :default "NewEnumerator0") (`Object To Set` :type "Object Object Reference"))
  (`BlackboardComponent.SetValueAsObject` (`self.BlackboardComponent`) (`KismetStringLibrary.Conv_StringToName` (`|GetEnumeratorNameAsString` `ObjectType Name`)) `Object To Set`))

(fn `SetStartingValues`
  (params (ShouldWander :type Boolean) (WanderDurationMax :type "Float (double-precision)") (WanderDurationMin :type "Float (double-precision)") (CanDropToTarget :type Boolean) (AcceptanceLengthForDrop :type "Float (double-precision)"))
  (`|ExecutionSequence`
    (:`then_0`
      (`self.SetBlackBoardBool` "NewEnumerator4" ShouldWander))
    (:`then_1`
      (`self.SetBlackBoardFloat` "NewEnumerator3" WanderDurationMax))
    (:`then_2`
      (`self.SetBlackBoardFloat` "NewEnumerator2" WanderDurationMin))
    (:`then_3`
      (`self.SetBlackBoardBool` "NewEnumerator3" CanDropToTarget))
    (:`then_4`
      (`self.SetBlackBoardFloat` "NewEnumerator0" AcceptanceLengthForDrop))))

(fn `UserConstructionScript`)